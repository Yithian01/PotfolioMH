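; Great sword weapon that overrides the parent weapon's charge attack, combo attack and dodge actions to play animation montages on the owning BP_Player.
; Each action calls an S2M RPC with a montage section chosen from charge time, combo count or four-way dodge direction.
; Charge level thresholds come from a lazily cached PDA_MeleeWeapon data asset.
; A completed combo montage calls back to the player to reset the combo count.
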(event EventBeginPlay
  (|CallParentFunction) ; This node is disabled and will not be called.\nDrag off pins to build functionality.
)

(event Collision|EventActorBeginOverlap
  (params (OtherActor :type Actor%20Object%20Reference))
  (|CallParentFunction OtherActor) ; This node is disabled and will not be called.\nDrag off pins to build functionality.
)

(event EventTick
  (params (DeltaSeconds :type Float%20%28single-precision%29))
  (|CallParentFunction DeltaSeconds) ; This node is disabled and will not be called.\nDrag off pins to build functionality.
)

(event Custom|S2M_PlayChargeStartMontage
  ;[0.15 0.15 0.15 0.5] StartChargeLoop
  (bind _asbp_player (Utilities|Casting|CastToBP_Player (Components|GetOwner)))
  (Animation|Montage|PlayMontage (Variables|/Script/Engine.Character|GetMesh _asbp_player) "/Game/InGame/Blueprints/Weapon/Animations/OLD_GreatSword/AM_GreatSword_Charge.AM_GreatSword_Charge" 1.0 0.0 "Charge_Start"))

(event Custom|S2M_PlayDodgeMontage
  (params (SectionName :type Name))
  ;[0.15 0.15 0.15 0.5] Dodge
  (bind _asbp_player (Utilities|Casting|CastToBP_Player (Components|GetOwner)))
  (Animation|Montage|PlayMontage (Variables|/Script/Engine.Character|GetMesh _asbp_player) "/Game/InGame/Blueprints/Weapon/Animations/OLD_GreatSword/AM_GreatSword_Dodge.AM_GreatSword_Dodge" 1.0 0.0 SectionName))

(event Custom|S2M_PlayComboAttackMontage
  (params (SectionName :type Name))
  ;[0.15 0.15 0.15 0.5] ComboAttack
  (bind _asbp_player (Utilities|Casting|CastToBP_Player (Components|GetOwner)))
  (Animation|Montage|PlayMontage (Variables|/Script/Engine.Character|GetMesh _asbp_player) "/Game/InGame/Blueprints/Weapon/Animations/OLD_GreatSword/AM_GreatSword_Combo.AM_GreatSword_Combo" 1.0 0.0 SectionName
    (:OnCompleted
      (Default|C2SInitalizeComboCount _asbp_player))))

(event Custom|S2M_PlayChargeAttackMontage
  (params (SectionName :type Name))
  ;[0.15 0.15 0.15 0.5] StartChargeAttack
  (bind _asbp_player (Utilities|Casting|CastToBP_Player (Components|GetOwner)))
  (Animation|Montage|PlayMontage (Variables|/Script/Engine.Character|GetMesh _asbp_player) "/Game/InGame/Blueprints/Weapon/Animations/OLD_GreatSword/AM_GreatSword_Charge.AM_GreatSword_Charge" 1.0 0.0 SectionName))

(fn ConstructionScript
  (|CallParentFunction))

(fn StartChargeAttack
  (|CallParentFunction)
  (CallFunction|S2MPlayChargeStartMontage))

(fn StartAttack
  (|CallParentFunction))

(fn GetCastingWeaponData
  (Utilities|IsValid (Variables|Default|GetGreateSwordData)
    (:Is%20Valid
      (return (Variables|Default|GetGreateSwordData)))
    (:Is%20Not%20Valid
      (Utilities|IsValid (Variables|Default|GetWeaponData)
        (:Is%20Valid
          (bind _aspda_melee_weapon (Utilities|Casting|CastToPDA_MeleeWeapon (Variables|Default|GetWeaponData)))
          (bind _output_get (Variables|Default|SetGreateSwordData _aspda_melee_weapon))
          (return _output_get))))))

(fn GetSectionNamebyCounter
  (params (ComboCount :type Integer))
  (return (Utilities|String|StringToName (Utilities|String|Append "Combo_Level" "_" (Utilities|String|ToString(Integer) ComboCount)))))

(fn GetSectionNamebyChargeTime
  (params (ChargeTime :type Float%20%28double-precision%29))
  (Utilities|FlowControl|Sequence
    (:then_0
      (if (not (>= ChargeTime (Variables|/Game/InGame/Datas/PDA/Weapon/PDA_MeleeWeapon.PDA_MeleeWeapon_C|GetChargeLevel2Time (Interal|GetCastingWeaponData))))
        (return "Charge_Level_1")))
    (:then_2
      (if (>= ChargeTime (Variables|/Game/InGame/Datas/PDA/Weapon/PDA_MeleeWeapon.PDA_MeleeWeapon_C|GetChargeLevel3Time (Interal|GetCastingWeaponData)))
        (return "Charge_Level_3")
        (else
          (return "Charge_Level_2"))))))

(fn ReleaseChargeAttack
  (params (ChargeTime :type Float%20%28double-precision%29))
  (|CallParentFunction ChargeTime)
  (bind _sectionname (Interal|GetSectionNamebyChargeTime ChargeTime))
  (CallFunction|S2MPlayChargeAttackMontage _sectionname))

(fn StartComboAttack
  (params (ComboCount :type Integer))
  (|CallParentFunction ComboCount)
  (CallFunction|S2MPlayComboAttackMontage (Interal|GetSectionNamebyCounter ComboCount)))

(fn StartDodge
  (|CallParentFunction)
  (bind _asbp_player (Utilities|Casting|CastToBP_Player (Components|GetOwner)))
  (LocalVariables|SetLocalDodgeDirection (Default|GetActorDirection _asbp_player))
  (Utilities|FlowControl|Sequence
    (:then_0
      (if (|((Angle>=(0-45))&&(Angle<=45)) (LocalVariables|GetLocalDodgeDirection))
        (LocalVariables|SetSectionName "Forward")))
    (:then_1
      (if (|((Angle>45)&&(Angle<135)) (LocalVariables|GetLocalDodgeDirection))
        (LocalVariables|SetSectionName "Right")))
    (:then_2
      (if (|((Angle>=135)||(Angle<=(0-135))) (LocalVariables|GetLocalDodgeDirection))
        (LocalVariables|SetSectionName "Back")))
    (:then_3
      (if (|((Angle>(0-135))&&(Angle<(0-45))) (LocalVariables|GetLocalDodgeDirection))
        (LocalVariables|SetSectionName "Left")))
    (:then_4
      (CallFunction|S2MPlayDodgeMontage (LocalVariables|GetSectionName)))))