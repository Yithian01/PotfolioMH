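; AN_Attack is an animation notify that deals melee-style area damage when an attack animation reaches it.
; It runs a single-hit sphere trace for Pawn objects from the mesh location along the mesh component's forward vector, ignoring the owner and drawing timed debug shapes.
; If the hit actor is a BP_InGameCharacter, it applies fixed damage to it, with no instigator or damage causer set.
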(fn `Received_Notify`
  (params (MeshComp :type "SkeletalMeshComponent Object Reference") (Animation :type "AnimSequenceBase Object Reference") (EventReference :type "AnimNotifyEventReference Structure (by ref)"))
  (returns (ReturnValue :type Boolean))
  (bind _returnvalue (`SceneComponent.K2_GetComponentLocation` MeshComp))
  (bind _outhit (`KismetSystemLibrary.SphereTraceSingleForObjects` _returnvalue (+ _returnvalue (* (`SceneComponent.GetForwardVector` MeshComp) 300.0)) 300.0 (`|MakeArray` "ObjectTypeQuery3" :!type "EObjectTypeQuery Enum") false (`|MakeArray` (`ActorComponent.GetOwner` MeshComp)) "ForDuration" false))
  (bind _asbp_in_game_character (cast `/Game/InGame/Blueprints/BP_InGameCharacter` (`.HitActor` (`GameplayStatics.BreakHitResult` _outhit))))
  (`GameplayStatics.ApplyDamage` _asbp_in_game_character 100.0)
  (return false))