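; BP_InGameCharacter is a base character Blueprint for in-game combatants, providing shared damage and attack state.
; PointDamage events call an empty TakeDamageProcess hook unless the invincibility flag is set, and EnableAttack turns on an attack-enable flag.
; GetForwardArc uses a dot-product math expression to test whether a target location lies within roughly 45 degrees of the actor's forward vector.
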(event Custom|EnableAttack
  (Variables|Default|SetbIsEnableAttack true))

(event Game|Damage|EventPointDamage
  (params (Damage :type Float%20%28single-precision%29) (DamageType :type Damage%20Type%20Object%20Reference) (HitLocation :type Vector :default "0, 0, 0") (HitNormal :type Vector :default "0, 0, 0") (HitComponent :type Primitive%20Component%20Object%20Reference) (BoneName :type Name :default "None") (ShotFromDirection :type Vector :default "0, 0, 0") (InstigatedBy :type Controller%20Object%20Reference) (DamageCauser :type Actor%20Object%20Reference) (HitInfo :type Hit%20Result%20Structure%20%28by%20ref%29))
  (if (not (Variables|Default|GetbIsInvincible))
    (CallFunction|TakeDamageProcess Damage)))

(event EventBeginPlay)

(fn ConstructionScript)

(fn GetForwardArc
  (params (TargetLocation :type Vector))
  (bind _returnvalue (Transformation|GetActorLocation))
  (bind _returnvalue_2 (Transformation|GetActorForwardVector))
  (bind _returnvalue_3 (- TargetLocation _returnvalue))
  (bind _returnvalue_4 (Math|Vector|Normalize _returnvalue_3))
  (return (|((((DX*FX)+(DY*FY))+(DZ*FZ))>=0.707000) (.x _returnvalue_4) (.x _returnvalue_2) (.y _returnvalue_4) (.y _returnvalue_2) (.z _returnvalue_4) (.z _returnvalue_2))))

(fn SetInvincible
  (params (bIsInvincible :type Boolean))
  (Variables|Default|SetbIsInvincible bIsInvincible))

(fn GetInvincible
  (return (Variables|Default|GetbIsInvincible)))

(fn TakeDamageProcess
  (params (AppliedDamage :type Float%20%28double-precision%29)))