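; Player stat component that manages stamina for running and dodging and reports HP and stamina changes.
; Starting and stopping a run swap one looping timer handle between periodic drain and regeneration capped at max.
; When stamina runs too low, it stops the run and resets walk speed on the owning BP_Player.
; Change and refresh functions broadcast current and max values through player stat events.
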(event `OnStartRun`
  (if (`KismetSystemLibrary.K2_IsValidTimerHandle` (`self.StaminaHandle`))
    (`KismetSystemLibrary.K2_ClearAndInvalidateTimerHandle` (`self.StaminaHandle`)))
  (bind _returnvalue (`KismetSystemLibrary.K2_SetTimerDelegate` (delegate `HandleStartRun`) 1.0 true))
  (`self.ConsumeStamina` 1.0)
  (set `self.StaminaHandle` _returnvalue))

(event `HandleStartRun`
  (if (`self.CanRun` 1.0)
    (`self.ConsumeStamina` 2.0)
    (else
      (`self.OnStopRun`)
      (bind _asbp_player (cast `/Game/InGame/Blueprints/Player/BP_Player` (`self.GetOwner`)))
      (`/Game/InGame/Blueprints/Player/BP_Player.ChangeMaxWalkSpeed` _asbp_player false))))

(event `OnStopRun`
  (if (`KismetSystemLibrary.K2_IsValidTimerHandle` (`self.StaminaHandle`))
    (`KismetSystemLibrary.K2_ClearAndInvalidateTimerHandle` (`self.StaminaHandle`)))
  (bind _returnvalue (`KismetSystemLibrary.K2_SetTimerDelegate` (delegate `HandleStaminaHeal`) 0.5 true))
  (set `self.StaminaHandle` _returnvalue))

(event `HandleStaminaHeal`
  (`self.StaminaHeal` 1.0))

(fn `CanDodge`
  (params (LessStamina :type "Float (double-precision)"))
  (returns (CanDodge :type Boolean))
  (return (> (- (`self.CurrentStamina`) LessStamina) 0.0)))

(fn `CanRun`
  (params (LessStamina :type "Float (double-precision)"))
  (returns (ReturnValue :type Boolean))
  (return (> (- (`self.CurrentStamina`) LessStamina) 0.0)))

(fn `ConsumeStamina`
  (params (UseStamina :type "Float (double-precision)"))
  (set `self.CurrentStamina` (- (`self.CurrentStamina`) UseStamina)))

(fn `OnChanedStamina`
  (`parent.OnChanedStamina`)
  (`self.OnPlayerStaminaChanged` (`self.CurrentStamina`) (`self.MaxStamina`)))

(fn `OnChangedHp`
  (`parent.OnChangedHp`)
  (`self.OnPlayerHpChanged` (`self.CurrentHp`) (`self.MaxHp`)))

(fn `RefreshHealth`
  (`self.OnChangedHp`))

(fn `RefreshStamina`
  (`self.OnPlayerStaminaChanged` (`self.CurrentStamina`) (`self.MaxStamina`)))

(fn `StaminaHeal`
  (params (HealingPerSeconed :type "Float (double-precision)"))
  (set `self.CurrentStamina` (`KismetMathLibrary.FMin` (+ HealingPerSeconed (`self.CurrentStamina`)) (`self.MaxStamina`))))

(fn `TakeDamage`
  (params (AppliedDamage :type "Float (double-precision)"))
  (returns (bIsDead :type Boolean))
  (bind _bisdead (`parent.TakeDamage` AppliedDamage))
  (return _bisdead))