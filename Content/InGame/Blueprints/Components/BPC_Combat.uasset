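; Combat component that runs an enum-based state machine for attacks, combos, charge attacks, dodges and hit reactions, delegating execution to the equipped weapon.
; A hold timer separates tap attacks from charge attacks, which release with their held duration.
; Presses during a combo advance a counter one step ahead, consumed by CheckingComboAttack, with a reset timer per step.
; Dodging spends stamina through the stat component; CanPerformAction looks up state-action rules in a DataTable.
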(fn `BeginAttackInput`
  (if (`|EnumEquality` (`self.CombatState`) "NewEnumerator0")
    (set `self.bAttackInputHeld` true)
    (set `self.bChargeStarted` false)
    (set `self.ChargeStartTime` 0.0)
    (bind _returnvalue (`KismetSystemLibrary.K2_SetTimerDelegate` (`|CreateDelegate` :!event `StartCharge`) (`self.AttackHoldThreshold`)))
    (set `self.ChargeTimerHandle` _returnvalue)
    (else
      (return))))

(fn `CancelAttackInput`
  (bind _chargetimerhandle (`self.ChargeTimerHandle`))
  (`|ExecutionSequence`
    (:`then_0`
      (set `self.bAttackInputHeld` false))
    (:`then_1`
      (if (`KismetSystemLibrary.K2_IsValidTimerHandle` _chargetimerhandle)
        (`KismetSystemLibrary.K2_ClearAndInvalidateTimerHandle` _chargetimerhandle)))
    (:`then_2`
      (if (`self.bChargeStarted`)
        (`self.CancelCharge`)
        (else
          (return))))))

(fn `CancelCharge`
  (if (`|EnumEquality` (`self.CombatState`) "NewEnumerator2")
    (`self.FinishAction`)))

(fn `CanPerformAction`
  (params (ActionType :type "/Game/InGame/Datas/Enum/Combat/E_PlayerActionType Enum" :default "NewEnumerator0"))
  (returns (bIsEnableInput :type Boolean))
  (bind _returnvalue (`|GetDataTableRow` "/Game/InGame/Datas/DataTable/DT_CombatActionRule.DT_CombatActionRule" (`KismetStringLibrary.Conv_StringToName` (`KismetStringLibrary.Concat_StrStr` (`|GetEnumeratorNameAsString` (`self.CombatState`)) "_" (`|GetEnumeratorNameAsString` (`local.ActionType`)))))
    (:`then`
      (return (break `/Game/InGame/Datas/Struct/Combat/ST_CombatActionRule` _returnvalue)))
    (:`RowNotFound`
      (return false))))

(fn `CheckCombo`
  (if (!= (`self.CurrentComboCount`) (`self.PlayingComboCount`))
    (`|ExecutionSequence`
      (:`then_0`
        (bind _currentweapon (`/Game/InGame/Blueprints/Components/BPC_Equipment.GetCurrentWeapon` (`self.EquipmentComponentRef`)))
        (`/Game/InGame/Blueprints/Weapon/BP_WeaponBase.StartComboAttack` _currentweapon (`self.CurrentComboCount`))
        (set `self.PlayingComboCount` (`self.CurrentComboCount`)))
      (:`then_1`
        (set `self.CombatState` "NewEnumerator1")
        (bind _returnvalue (`KismetSystemLibrary.K2_SetTimerDelegate` (`|CreateDelegate` :!event `EndCombatAttack`) (`self.ComboResetTime`)))
        (set `self.ComboTimerHandle` _returnvalue)))))

(fn `CheckingComboAttack`
  (`self.CheckCombo`))

(fn `EndAttackInput`
  (bind _chargetimerhandle (`self.ChargeTimerHandle`))
  (`|ExecutionSequence`
    (:`then_0`
      (set `self.bAttackInputHeld` false))
    (:`then_1`
      (if (`KismetSystemLibrary.K2_IsValidTimerHandle` _chargetimerhandle)
        (`KismetSystemLibrary.K2_ClearAndInvalidateTimerHandle` _chargetimerhandle)))
    (:`then_2`
      (if (`self.bChargeStarted`)
        (`self.ReleaseCharge`)
        (else
          (`self.StartSingleOrComboAttack`))))))

(fn `EndCombatAttack`
  (`|ExecutionSequence`
    (:`then_0`
      (`self.FinishAction`)
      (set `self.CurrentComboCount` 0)
      (set `self.PlayingComboCount` 0))
    (:`then_1`
      (if (`KismetSystemLibrary.K2_IsValidTimerHandle` (`self.ComboTimerHandle`))
        (`KismetSystemLibrary.K2_ClearAndInvalidateTimerHandle` (`self.ComboTimerHandle`))))))

(fn `EndDodge`
  (if (`|EnumEquality` (`self.CombatState`) "NewEnumerator3")
    (`self.SetIdleState`)))

(fn `FinishAction`
  (`self.SetIdleState`))

(fn `FinishCombatState`
  (`self.EndCombatAttack`))

(fn `HitReaction`
  (`self.EndCombatAttack`)
  (set `self.CombatState` "NewEnumerator4"))

(fn `InitializeCombat`
  (params (EquipmentComponent :type "/Game/InGame/Blueprints/Components/BPC_Equipment Object Reference") (StatComponent :type "/Game/InGame/Blueprints/Components/BPC_PlayerStatComponent Object Reference"))
  (`|ExecutionSequence`
    (:`then_0`
      (set `self.EquipmentComponentRef` (`local.EquipmentComponent`))
      (set `self.StatComponentRef` (`local.StatComponent`))
      (set `self.CanComboAttack` true))))

(fn `InitializeComboAttack`
  (`self.EndCombatAttack`))

(fn `ReleaseCharge`
  (if (`|EnumEquality` (`self.CombatState`) "NewEnumerator2")
    (bind _currentweapon (`/Game/InGame/Blueprints/Components/BPC_Equipment.GetCurrentWeapon` (`self.EquipmentComponentRef`)))
    (`/Game/InGame/Blueprints/Weapon/BP_WeaponBase.ReleaseChargeAttack` _currentweapon (- (`KismetSystemLibrary.GetGameTimeInSeconds`) (`self.ChargeStartTime`)))
    (`self.EndCombatAttack`)))

(fn `SetIdleState`
  (set `self.CombatState` "NewEnumerator0"))

(fn `StartCharge`
  (if (`self.bAttackInputHeld`)
    (set `self.CombatState` "NewEnumerator2")
    (set `self.bChargeStarted` true)
    (set `self.ChargeStartTime` (`KismetSystemLibrary.GetGameTimeInSeconds`))
    (bind _currentweapon (`/Game/InGame/Blueprints/Components/BPC_Equipment.GetCurrentWeapon` (`self.EquipmentComponentRef`)))
    (`/Game/InGame/Blueprints/Weapon/BP_WeaponBase.StartChargeAttack` _currentweapon)
    (else
      (return))))

(fn `StartComboAttack`
  (if (`|EnumEquality` (`self.CombatState`) "NewEnumerator0")
    (`|ExecutionSequence`
      (:`then_0`
        (bind _result (`/Engine/EditorBlueprintResources/StandardMacros.IncrementInt` (`self.CurrentComboCount`))
          (:`  `
            (set `self.PlayingComboCount` _result))))
      (:`then_1`
        (bind _currentweapon (`/Game/InGame/Blueprints/Components/BPC_Equipment.GetCurrentWeapon` (`self.EquipmentComponentRef`)))
        (`/Game/InGame/Blueprints/Weapon/BP_WeaponBase.StartComboAttack` _currentweapon (`self.CurrentComboCount`)))
      (:`then_2`
        (set `self.CombatState` "NewEnumerator1")
        (bind _returnvalue (`KismetSystemLibrary.K2_SetTimerDelegate` (`|CreateDelegate` :!event `EndCombatAttack`) (`self.ComboResetTime`)))
        (set `self.ComboTimerHandle` _returnvalue)))
    (elif (== (`self.CurrentComboCount`) (`self.PlayingComboCount`))
      (`/Engine/EditorBlueprintResources/StandardMacros.IncrementInt` (`self.CurrentComboCount`)))))

(fn `StartDodge`
  (if (`/Game/InGame/Blueprints/Components/BPC_PlayerStatComponent.CanDodge` (`self.StatComponentRef`) 30.0)
    (if (`|EnumInequality` (`self.CombatState`) "NewEnumerator3")
      (set `self.CombatState` "NewEnumerator3")
      (`/Game/InGame/Blueprints/Components/BPC_PlayerStatComponent.ConsumeStamina` (`self.StatComponentRef`) 30.0)
      (bind _currentweapon (`/Game/InGame/Blueprints/Components/BPC_Equipment.GetCurrentWeapon` (`self.EquipmentComponentRef`)))
      (`/Game/InGame/Blueprints/Weapon/BP_WeaponBase.StartDodge` _currentweapon))))

(fn `StartDodgeInput`
  (`self.StartDodge`))

(fn `StartSingleOrComboAttack`
  (if (`self.CanComboAttack`)
    (`self.StartComboAttack`)
    (else
      (set `self.CombatState` "NewEnumerator1")
      (bind _currentweapon (`/Game/InGame/Blueprints/Components/BPC_Equipment.GetCurrentWeapon` (`self.EquipmentComponentRef`)))
      (`/Game/InGame/Blueprints/Weapon/BP_WeaponBase.StartAttack` _currentweapon))))