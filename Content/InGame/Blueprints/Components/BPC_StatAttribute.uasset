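; Stat component holding HP, stamina, attack, defense and move speed, with InitializeStats setting their defaults.
; HP and stamina use RepNotify, routing current and max changes into OnChangedHp and OnChanedStamina, which are empty hooks.
; TakeDamage subtracts raw damage without using defense, but its branch condition is constant true, so it always zeroes HP and returns true.
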(fn `InitializeStats`
  (`|ExecutionSequence`
    (:`then_0`
      (bind _output_get (set `self.MaxHp` 100.0))
      (set `self.CurrentHp` _output_get))
    (:`then_1`
      (bind _output_get_2 (set `self.MaxStamina` 100.0))
      (set `self.CurrentStamina` _output_get_2))
    (:`then_2`
      (set `self.AttackPower` 0.0)
      (set `self.AttackSpeed` 0.0))
    (:`then_3`
      (set `self.DefensePower` 10.0))
    (:`then_4`
      (set `self.MoveSpeed` 400.0))))

(fn `OnChanedStamina`)

(fn `OnChangedHp`)

(fn `OnRep_CurrentHp`
  (`self.OnChangedHp`))

(fn `OnRep_CurrentStamina`
  (`self.OnChanedStamina`))

(fn `OnRep_MaxHp`
  (`self.OnChangedHp`))

(fn `OnRep_MaxStamina`
  (`self.OnChanedStamina`))

(fn `TakeDamage`
  (params (AppliedDamage :type "Float (double-precision)"))
  (returns (bIsDead :type Boolean))
  (locals (LocalCurrentHp :type "Float (double-precision)"))
  (set `local.LocalCurrentHp` (- (`self.CurrentHp`) AppliedDamage))
  (if true
    (set `self.CurrentHp` 0.0)
    (return true)
    (else
      (set `self.CurrentHp` (`local.LocalCurrentHp`))
      (return false))))