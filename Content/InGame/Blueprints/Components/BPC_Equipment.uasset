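; Player equipment component that tracks items by slot and handles the spawned weapon actor, attaching it to armed or unarmed sockets.
; Equip, unequip and swap functions move items between the slot map and inventory component, resolving ring slots and two-handed items.
; C2S events run these operations, then S2C events replay them for players not locally controlled on the caller.
; Change notifications fire only for the locally controlled player.
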(event `C2S_EquipmentItem`
  (params (TargetSlot :type "/Game/InGame/Datas/Enum/Item/E_EquipmentSlot Enum" :default "NewEnumerator0") (TargetItem :type "/Game/InGame/Datas/Struct/Item/ST_ItemInstance Structure") (StorageType :type "/Game/InGame/Datas/Enum/Item/E_StorageType Enum" :default "NewEnumerator0") (EquippedSlotType :type "/Game/InGame/Datas/Enum/Item/E_EquipmentSlot Enum" :default "NewEnumerator0"))
  ; 아이템 장착 or 옮기기(반지의 경우)
  (bind (_bsucceeded _equippedslot _equippeditem _itemstoragetype _itemequippedslottype) (`self.TryEquipItem` TargetSlot TargetItem StorageType EquippedSlotType))
  (if (not (`Pawn.IsLocallyControlled` (`self.GetOrCreatePlayer`)))
    (`self.S2C_EquipmentItem` _bsucceeded _equippedslot _equippeditem _itemstoragetype _itemequippedslottype)))

(event `S2C_EquipmentItem`
  (params (bSucceeded :type Boolean) (TargetSlot :type "/Game/InGame/Datas/Enum/Item/E_EquipmentSlot Enum" :default "NewEnumerator0") (TargetItem :type "/Game/InGame/Datas/Struct/Item/ST_ItemInstance Structure") (StorageType :type "/Game/InGame/Datas/Enum/Item/E_StorageType Enum" :default "NewEnumerator0") (EquippedSlotType :type "/Game/InGame/Datas/Enum/Item/E_EquipmentSlot Enum" :default "NewEnumerator0"))
  ; 아이템 장착 or 옮기기(반지의 경우)
  (if bSucceeded
    (`self.TryEquipItem` TargetSlot TargetItem StorageType EquippedSlotType)))

(event `C2S_UnequipItem`
  (params (TargetSlot :type "/Game/InGame/Datas/Enum/Item/E_EquipmentSlot Enum" :default "NewEnumerator0") (TargetItem :type "/Game/InGame/Datas/Struct/Item/ST_ItemInstance Structure"))
  ; UnequipItem
  (bind (_bissucceeded _unequipslot _unequipitem) (`self.TryUnequipItem` TargetSlot TargetItem))
  (if (not (`Pawn.IsLocallyControlled` (`self.GetOrCreatePlayer`)))
    (`self.S2C_UnEquipItem` _unequipslot _unequipitem)))

(event `S2C_UnequipItem`
  (params (TargetSlot :type "/Game/InGame/Datas/Enum/Item/E_EquipmentSlot Enum" :default "NewEnumerator0") (TargetItem :type "/Game/InGame/Datas/Struct/Item/ST_ItemInstance Structure"))
  ; UnequipItem
  (`self.TryUnequipItem` TargetSlot TargetItem))

(fn `CanEquipItem`
  (params (TargetSlot :type "/Game/InGame/Datas/Enum/Item/E_EquipmentSlot Enum" :default "NewEnumerator0") (TargetItem :type "/Game/InGame/Datas/Struct/Item/ST_ItemInstance Structure"))
  (returns (bCanEquip :type Boolean) (SwapSlot :type "/Game/InGame/Datas/Enum/Item/E_EquipmentSlot Enum"))
  (locals (LocalTargetSlot :type "/Game/InGame/Datas/Enum/Item/E_EquipmentSlot Enum"))
  (bind (_bsucceeded _findslot) (`self.FindCanEquipRingSlot` (`local.TargetSlot`)))
  (`|ExecutionSequence`
    (:`then_0`
      (set `local.LocalTargetSlot` _findslot)
      (if (not _bsucceeded)
        (return false "NewEnumerator0")))
    (:`then_1`
      (return (not (`BlueprintMapLibrary.Map_Contains` (`self.EquipmentItems`) (`local.LocalTargetSlot`))) (`local.LocalTargetSlot`)))))

(fn `CanReplaceToInventoryItem`
  (params (TargetSlot :type "/Game/InGame/Datas/Enum/Item/E_EquipmentSlot Enum" :default "NewEnumerator0") (TargetItem :type "/Game/InGame/Datas/Struct/Item/ST_ItemInstance Structure"))
  (returns (bCanReplace :type Boolean) (StartPoint :type "IntPoint Structure") (EquippedItem :type "/Game/InGame/Datas/Struct/Item/ST_ItemInstance Structure"))
  (locals (LocalFalseResult :type "IntPoint Structure" :default (struct :`X` -1 :`Y` -1)) (LocalEquippedItem :type "/Game/InGame/Datas/Struct/Item/ST_ItemInstance Structure"))
  (bind (_item _bsuceeded) (`self.GetEquipedItem` (`local.TargetSlot`)))
  (`/Engine/EditorBlueprintResources/StandardMacros.IsValid` (`self.InventoryComponentRef`)
    (:`Is Valid`
      (set `local.LocalEquippedItem` _item)
      (if _bsuceeded
        (bind (_bcanstore _startpoint) (`/Game/InGame/Blueprints/Components/BPC_InventoryComponent.FindFirstAvailableSlot` (`self.InventoryComponentRef`) (`local.LocalEquippedItem`) (`local.TargetItem`)))
        (if _bcanstore
          (return true _startpoint (`local.LocalEquippedItem`))
          (else
            (return false (`local.LocalFalseResult`))))
        (else
          (return false (`local.LocalFalseResult`)))))
    (:`Is Not Valid`
      (return false (`local.LocalFalseResult`)))))

(fn `DrawWeapon`
  (if (and (`KismetSystemLibrary.IsValid` (`self.CurrentWeapon`)) (not (`self.bIsWeaponDrawn`)))
    (bind _asbp_player (cast `/Game/InGame/Blueprints/Player/BP_Player` (`self.GetOwner`)))
    (bind _returnvalue (`Actor.K2_AttachToComponent` (`self.CurrentWeapon`) (`Character.Mesh` _asbp_player) (`/Game/InGame/Datas/PDA/Weapon/PDA_WeaponData.ArmedSocketName` (`self.WeaponData`)) "SnapToTarget" "SnapToTarget" "SnapToTarget" true))
    (set `self.bIsWeaponDrawn` _returnvalue)
    (else
      (return))))

(fn `EquippedItem`
  (params (NewItem :type "/Game/InGame/Datas/Struct/Item/ST_ItemInstance Structure"))
  (returns (bSucceeded :type Boolean) (EquippedSlot :type "/Game/InGame/Datas/Enum/Item/E_EquipmentSlot Enum") (HadReplaceItem :type Boolean) (ReplacedItem :type "/Game/InGame/Datas/Struct/Item/ST_ItemInstance Structure"))
  (locals (LocalTargetSlot :type "/Game/InGame/Datas/Enum/Item/E_EquipmentSlot Enum" :default "NewEnumerator0") (LocalPreviousItem :type "/Game/InGame/Datas/Struct/Item/ST_ItemInstance Structure") (LocalHadPreviousItem :type Boolean :default false))
  (bind (_item _bsuceeded) (`self.GetEquipedItem` (`local.LocalTargetSlot`)))
  (bind _aspda_equipment_definition (cast `/Game/InGame/Datas/PDA/Item/PDA_EquipmentDefinition` (`.ItemDefinition_9_88C99C9B4588673D38DD769AFBFB6841` (break `/Game/InGame/Datas/Struct/Item/ST_ItemInstance` NewItem)))
    (:`then`
      (bind _output_get (set `local.LocalTargetSlot` (`/Game/InGame/Datas/PDA/Item/PDA_EquipmentDefinition.EquipmentSlot` _aspda_equipment_definition)))
      (if (`self.CanReplaceToInventoryItem` _output_get (`local.NewItem`))
        (set `local.LocalPreviousItem` _item)
        (set `local.LocalHadPreviousItem` _bsuceeded)
        (`self.SetEquipmentItem` (`local.LocalTargetSlot`) (`local.NewItem`))
        (return true (`local.LocalTargetSlot`) (`local.LocalHadPreviousItem`) (`local.LocalPreviousItem`))
        (else
          (return true "NewEnumerator0" true))))
    (:`CastFailed`
      (return false "NewEnumerator0" false))))

(fn `FindCanEquipRingSlot`
  (params (SlotType :type "/Game/InGame/Datas/Enum/Item/E_EquipmentSlot Enum" :default "NewEnumerator0"))
  (returns (bSucceeded :type Boolean) (FindSlot :type "/Game/InGame/Datas/Enum/Item/E_EquipmentSlot Enum"))
  (if (`|EnumEquality` SlotType "NewEnumerator10")
    (`|ExecutionSequence`
      (:`then_0`
        (if (not (`.ReturnValue` (`BlueprintMapLibrary.Map_Find` (`self.EquipmentItems`) "NewEnumerator6")))
          (return true "NewEnumerator6")))
      (:`then_1`
        (if (`.ReturnValue` (`BlueprintMapLibrary.Map_Find` (`self.EquipmentItems`) "NewEnumerator7"))
          (return true "NewEnumerator6")
          (else
            (return true "NewEnumerator7")))))
    (else
      (return true (`local.SlotType`)))))

(fn `GetCurrentWeapon`
  (returns (CurrentWeapon :type "/Game/InGame/Blueprints/Weapon/BP_WeaponBase Object Reference"))
  (return (`self.CurrentWeapon`)))

(fn `GetEquipedItem`
  (params (Slot :type "/Game/InGame/Datas/Enum/Item/E_EquipmentSlot Enum" :default "NewEnumerator0"))
  (returns (Item :type "/Game/InGame/Datas/Struct/Item/ST_ItemInstance Structure") (bSuceeded :type Boolean))
  (bind (_value _returnvalue) (`BlueprintMapLibrary.Map_Find` (`self.EquipmentItems`) Slot))
  (return _value _returnvalue))

(fn `GetOrCreateInventoryComponent`
  (returns (InventoryComponentRef :type "/Game/InGame/Blueprints/Components/BPC_InventoryComponent Object Reference"))
  (`/Engine/EditorBlueprintResources/StandardMacros.IsValid` (`self.InventoryComponentRef`)
    (:`Is Valid`
      _)
    (:`Is Not Valid`
      (set `self.InventoryComponentRef` (`/Game/InGame/Blueprints/Player/BP_Player.InventoryComponent` (`self.GetorCreatePlayer`)))))
  (return (`self.InventoryComponentRef`)))

(fn `GetOrCreatePlayer`
  (returns (PlayerRef :type "/Game/InGame/Blueprints/Player/BP_Player Object Reference"))
  (`/Engine/EditorBlueprintResources/StandardMacros.IsValid` (`self.PlayerRef`)
    (:`Is Valid`
      _)
    (:`Is Not Valid`
      (bind _asbp_player (cast `/Game/InGame/Blueprints/Player/BP_Player` (`self.GetOwner`)))
      (set `self.PlayerRef` _asbp_player)))
  (return (`self.PlayerRef`)))

(fn `InitializeWeapon`
  (params (WeaponData :type "/Game/InGame/Datas/PDA/Weapon/PDA_WeaponData Object Reference") (AttachParent :type "SceneComponent Object Reference"))
  (`/Engine/EditorBlueprintResources/StandardMacros.IsValid` WeaponData
    (:`Is Valid`
      (bind _output_get (set `self.WeaponData` WeaponData))
      (set `self.WeaponType` (`/Game/InGame/Datas/PDA/Weapon/PDA_WeaponData.WeaponType` _output_get))
      (bind _returnvalue (`|SpawnActorFromClass` (`/Game/InGame/Datas/PDA/Weapon/PDA_WeaponData.WeaponClass` (`self.WeaponData`)) (`KismetMathLibrary.MakeTransform` (0.0 0.0 0.0)) "AdjustIfPossibleButAlwaysSpawn" "MultiplyWithRoot" (`self.GetOwner`) (`self.WeaponData`) null))
      (bind _output_get_2 (set `self.CurrentWeapon` _returnvalue))
      (bind _returnvalue_2 (`Actor.K2_AttachToComponent` _output_get_2 (`local.AttachParent`) (`/Game/InGame/Datas/PDA/Weapon/PDA_WeaponData.UnarmedSocketName` (`self.WeaponData`)) "SnapToTarget" "SnapToTarget" "SnapToTarget" true))
      (set `self.bWeaponInitialized` _returnvalue_2))))

(fn `IsTwoHandedItem`
  (params (TargetItem :type "/Game/InGame/Datas/Struct/Item/ST_ItemInstance Structure"))
  (returns (bIsTwohanded :type Boolean))
  (bind (_itemuid _itemdefinition) (break `/Game/InGame/Datas/Struct/Item/ST_ItemInstance` TargetItem))
  (`/Engine/EditorBlueprintResources/StandardMacros.IsValid` _itemdefinition
    (:`Is Valid`
      (bind _aspda_equipment_definition (cast `/Game/InGame/Datas/PDA/Item/PDA_EquipmentDefinition` _itemdefinition))
      (return (`/Game/InGame/Datas/PDA/Item/PDA_EquipmentDefinition.bIsTwoHanded` _aspda_equipment_definition)))
    (:`Is Not Valid`
      (return false))))

(fn `RefreshItem`
  (params (ChangedSlot :type "/Game/InGame/Datas/Enum/Item/E_EquipmentSlot Enum" :default "NewEnumerator0") (EquipmentItem :type "/Game/InGame/Datas/Struct/Item/ST_ItemInstance Structure") (bIsTwoHanded :type Boolean))
  (if (`Pawn.IsLocallyControlled` (`self.GetOrCreatePlayer`))
    (`self.OnEquipmentChanged` ChangedSlot EquipmentItem bIsTwoHanded)))

(fn `SetEquipmentItem`
  (params (Slot :type "/Game/InGame/Datas/Enum/Item/E_EquipmentSlot Enum" :default "NewEnumerator0") (Item :type "/Game/InGame/Datas/Struct/Item/ST_ItemInstance Structure"))
  (`BlueprintMapLibrary.Map_Add` (`self.EquipmentItems`) Slot Item))

(fn `SheatheWeapon`
  (if (and (`KismetSystemLibrary.IsValid` (`self.CurrentWeapon`)) (`self.bIsWeaponDrawn`))
    (bind _asbp_player (cast `/Game/InGame/Blueprints/Player/BP_Player` (`self.GetOwner`)))
    (`Actor.K2_AttachToComponent` (`self.CurrentWeapon`) (`Character.Mesh` _asbp_player) (`/Game/InGame/Datas/PDA/Weapon/PDA_WeaponData.UnarmedSocketName` (`self.WeaponData`)) "SnapToTarget" "SnapToTarget" "SnapToTarget" true)
    (set `self.bIsWeaponDrawn` false)
    (else
      (return))))

(fn `SwapEquipToEquipItem`
  (params (TargetSlot :type "/Game/InGame/Datas/Enum/Item/E_EquipmentSlot Enum" :default "NewEnumerator0") (OriginSlot :type "/Game/InGame/Datas/Enum/Item/E_EquipmentSlot Enum" :default "NewEnumerator0") (OriginItem :type "/Game/InGame/Datas/Struct/Item/ST_ItemInstance Structure"))
  (returns (bSucceeded :type Boolean))
  (locals (LocalTargetItem :type "/Game/InGame/Datas/Struct/Item/ST_ItemInstance Structure"))
  (bind (_value _returnvalue) (`BlueprintMapLibrary.Map_Find` (`self.EquipmentItems`) (`local.TargetSlot`)))
  (`|ExecutionSequence`
    (:`then_0`
      (if (`|EnumEquality` (`local.OriginSlot`) "NewEnumerator0")
        (return false)))
    (:`then_1`
      (set `local.LocalTargetItem` _value)
      (if _returnvalue
        (`self.SetEquipmentItem` (`local.TargetSlot`) (`local.OriginItem`))
        (`self.RefreshItem` (`local.TargetSlot`) (`local.OriginItem`))
        (`self.SetEquipmentItem` (`local.OriginSlot`) (`local.LocalTargetItem`))
        (`self.RefreshItem` (`local.OriginSlot`) (`local.LocalTargetItem`))
        (return true)
        (else
          (`self.SetEquipmentItem` (`local.TargetSlot`) (`local.OriginItem`))
          (`self.RefreshItem` (`local.TargetSlot`) (`local.OriginItem`))
          ; TODO - 내부 함수로 분리
          (`self.UnequipItem` (`local.OriginSlot`) (`local.OriginItem`))
          (`self.RefreshItem` (`local.OriginSlot`))
          (return true))))))

(fn `TryEquipItem`
  (params (TargetSlot :type "/Game/InGame/Datas/Enum/Item/E_EquipmentSlot Enum" :default "NewEnumerator0") (TargetItem :type "/Game/InGame/Datas/Struct/Item/ST_ItemInstance Structure") (StorageType :type "/Game/InGame/Datas/Enum/Item/E_StorageType Enum" :default "NewEnumerator0") (EquippedSlotType :type "/Game/InGame/Datas/Enum/Item/E_EquipmentSlot Enum" :default "NewEnumerator0"))
  (returns (bSucceeded :type Boolean) (EquippedSlot :type "/Game/InGame/Datas/Enum/Item/E_EquipmentSlot Enum") (EquippedItem :type "/Game/InGame/Datas/Struct/Item/ST_ItemInstance Structure") (ItemStorageType :type "/Game/InGame/Datas/Enum/Item/E_StorageType Enum") (ItemEquippedSlotType :type "/Game/InGame/Datas/Enum/Item/E_EquipmentSlot Enum"))
  (locals (LocalTargetSlot :type "/Game/InGame/Datas/Enum/Item/E_EquipmentSlot Enum") (LocalOriginEquipmentItem :type "/Game/InGame/Datas/Struct/Item/ST_ItemInstance Structure"))
  (bind _inventorycomponentref (`self.GetOrCreateInventoryComponent`))
  (bind (_value _returnvalue) (`BlueprintMapLibrary.Map_Find` (`self.EquipmentItems`) (`local.LocalTargetSlot`)))
  (bind (_bcanequip _swapslot) (`self.CanEquipItem` (`local.TargetSlot`) (`local.TargetItem`)))
  (if (`|EnumEquality` (`local.StorageType`) "NewEnumerator1")
    (bind _bsucceeded (`self.SwapEquipToEquipItem` (`local.TargetSlot`) (`local.EquippedSlotType`) (`local.TargetItem`)))
    (return _bsucceeded (`local.TargetSlot`) (`local.TargetItem`) (`local.StorageType`) (`local.EquippedSlotType`))
    (else
      (set `local.LocalTargetSlot` _swapslot)
      (if _bcanequip
        (bind _bissucceeded (`/Game/InGame/Blueprints/Components/BPC_InventoryComponent.RemoveItem` (`self.GetOrCreateInventoryComponent`) (`local.TargetItem`)))
        (if _bissucceeded
          (`self.SetEquipmentItem` (`local.LocalTargetSlot`) (`local.TargetItem`))
          (`self.RefreshItem` (`local.LocalTargetSlot`) (`local.TargetItem`) (`self.IsTwoHandedItem` (`local.TargetItem`)))
          (return true (`local.LocalTargetSlot`) (`local.TargetItem`) (`local.StorageType`) (`local.EquippedSlotType`))
          (else
            (return false (`local.TargetSlot`) (`local.TargetItem`) (`local.StorageType`) (`local.EquippedSlotType`))))
        (else
          (set `local.LocalOriginEquipmentItem` _value)
          (if _returnvalue
            (`self.SetEquipmentItem` (`local.LocalTargetSlot`) (`local.TargetItem`))
            (`self.RefreshItem` (`local.LocalTargetSlot`) (`local.TargetItem`) (`self.IsTwoHandedItem` (`local.TargetItem`)))
            (`/Game/InGame/Blueprints/Components/BPC_InventoryComponent.RemoveItem` (`self.GetOrCreateInventoryComponent`) (`local.TargetItem`))
            (bind _succeeded_ (`/Game/InGame/Blueprints/Components/BPC_InventoryComponent.AddItem` _inventorycomponentref (`local.LocalOriginEquipmentItem`) (`local.TargetItem`)))
            (`/Game/InGame/Blueprints/Components/BPC_InventoryComponent.RefreshInventory` _inventorycomponentref)
            (return _succeeded_ (`local.LocalTargetSlot`) (`local.TargetItem`) (`local.StorageType`) (`local.EquippedSlotType`))
            (else
              (return false "NewEnumerator0" (struct) "NewEnumerator0" "NewEnumerator0"))))))))

(fn `TryUnequipItem`
  (params (TargetSlot :type "/Game/InGame/Datas/Enum/Item/E_EquipmentSlot Enum" :default "NewEnumerator0") (TargetItem :type "/Game/InGame/Datas/Struct/Item/ST_ItemInstance Structure") (IgnoreItem :type "/Game/InGame/Datas/Struct/Item/ST_ItemInstance Structure"))
  (returns (bIsSucceeded :type Boolean) (UnequipSlot :type "/Game/InGame/Datas/Enum/Item/E_EquipmentSlot Enum") (UnequipItem :type "/Game/InGame/Datas/Struct/Item/ST_ItemInstance Structure"))
  (bind _succeeded_ (`/Game/InGame/Blueprints/Components/BPC_InventoryComponent.AddItem` (`self.GetOrCreateInventoryComponent`) TargetItem IgnoreItem))
  (if _succeeded_
    (`/Game/InGame/Blueprints/Components/BPC_InventoryComponent.RefreshInventory` (`self.GetOrCreateInventoryComponent`))
    (bind (_bsucceeded _unequipslot _unequipitem _bistwohanded) (`self.UnequipItem` (`local.TargetSlot`) (`local.TargetItem`)))
    (if _bsucceeded
      (`self.RefreshItem` _unequipslot _unequipitem _bistwohanded)
      (return true (`local.TargetSlot`) (`local.TargetItem`)))
    (else
      (return false "NewEnumerator0"))))

(fn `UnequipItem`
  (params (TargetSlot :type "/Game/InGame/Datas/Enum/Item/E_EquipmentSlot Enum" :default "NewEnumerator0") (TargetItem :type "/Game/InGame/Datas/Struct/Item/ST_ItemInstance Structure"))
  (returns (bSucceeded :type Boolean) (UnequipSlot :type "/Game/InGame/Datas/Enum/Item/E_EquipmentSlot Enum") (UnequipItem :type "/Game/InGame/Datas/Struct/Item/ST_ItemInstance Structure") (bIsTwoHanded :type Boolean))
  (locals (LocalUnequipItem :type "/Game/InGame/Datas/Struct/Item/ST_ItemInstance Structure") (LocalbIsTwoHanded :type Boolean :default false) (LocalUnequipResult :type Boolean :default false))
  (bind (_value _returnvalue) (`BlueprintMapLibrary.Map_Find` (`self.EquipmentItems`) (`local.TargetSlot`)))
  (`|ExecutionSequence`
    (:`then_0`
      (bind _aspda_equipment_definition (cast `/Game/InGame/Datas/PDA/Item/PDA_EquipmentDefinition` (`.ItemDefinition_9_88C99C9B4588673D38DD769AFBFB6841` (break `/Game/InGame/Datas/Struct/Item/ST_ItemInstance` (`local.TargetItem`)))))
      (set `local.LocalbIsTwoHanded` (`/Game/InGame/Datas/PDA/Item/PDA_EquipmentDefinition.bIsTwoHanded` _aspda_equipment_definition)))
    (:`then_1`
      (if _returnvalue
        (set `local.LocalUnequipItem` _value)
        (bind _returnvalue_2 (`BlueprintMapLibrary.Map_Remove` (`self.EquipmentItems`) (`local.TargetSlot`)))
        (set `local.LocalUnequipResult` _returnvalue_2)
        (else
          (return false (`local.TargetSlot`) (struct) false))))
    (:`then_2`
      (if (`local.LocalbIsTwoHanded`)
        (`BlueprintMapLibrary.Map_Remove` (`self.EquipmentItems`) "NewEnumerator11")
        (return (`local.LocalUnequipResult`) (`local.TargetSlot`) (struct) (`local.LocalbIsTwoHanded`))
        (else
          (return (`local.LocalUnequipResult`) (`local.TargetSlot`) (struct) (`local.LocalbIsTwoHanded`)))))))