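; Monster stat component that extends a parent stat component to report HP changes as boss health updates.
; The OnChangedHp override runs the parent logic, then broadcasts current and max HP through the OnBossHpChanged dispatcher.
; RefreshHealth calls OnChangedHp to re-send the current values on demand, while TakeDamage simply passes through to the parent implementation.
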(fn `OnChangedHp`
  (`parent.OnChangedHp`)
  (`self.OnBossHpChanged` (`self.CurrentHp`) (`self.MaxHp`)))

(fn `RefreshHealth`
  (`self.OnChangedHp`))

(fn `TakeDamage`
  (params (AppliedDamage :type "Float (double-precision)"))
  (returns (bIsDead :type Boolean))
  (bind _bisdead (`parent.TakeDamage` AppliedDamage))
  (return _bisdead))