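; Player equipment component that equips, swaps and unequips items by UID in a slot map, exchanging them with the inventory component.
; Slot logic resolves ring pairs and one- or two-handed weapons, checking inventory space for displaced weapons.
; The server runs each request, then the remote owning client replays it via S2C RPC, firing a local change event.
; The server path also updates helmet and weapon meshes and the weapon behavior state.
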(event Custom|S2C_EquipmentItem
  (params (bSucceeded :type Boolean) (TargetSlot :type E_EquipmentSlot%20Enum :default "NewEnumerator0") (StorageType :type E_StorageType%20Enum :default "NewEnumerator0") (EquippedSlotType :type E_EquipmentSlot%20Enum :default "NewEnumerator0") (EquippedItemUID :type Guid%20Structure))
  ;[0.15 0.15 0.15 0.5] 아이템 장착 or 옮기기(반지의 경우)
  (Equipment|Action|TryEquipItem TargetSlot StorageType EquippedSlotType EquippedItemUID))

(event Custom|S2C_UnequipItem
  (params (TargetSlot :type E_EquipmentSlot%20Enum :default "NewEnumerator0") (TargetItemUID :type Guid%20Structure))
  ;[0.15 0.15 0.15 0.5] UnequipItem
  (Equipment|Action|TryUnequipItem TargetSlot TargetItemUID))

(event Custom|C2S_EquipmentItem
  (params (TargetSlot :type E_EquipmentSlot%20Enum :default "NewEnumerator0") (StorageType :type E_StorageType%20Enum :default "NewEnumerator0") (EquippedSlotType :type E_EquipmentSlot%20Enum :default "NewEnumerator0") (TargetItemUID :type Guid%20Structure))
  ;[0.15 0.15 0.15 0.5] 아이템 장착 or 옮기기(반지의 경우)
  (bind (_bsucceeded _equippedslot _itemstoragetype _itemequippedslottype _equippeditemuid) (Equipment|Action|TryEquipItem TargetSlot StorageType EquippedSlotType TargetItemUID))
  (if _bsucceeded
    (Equipment|Visual|Action|HandleUpdateEquipmentVisual _equippedslot)
    (if (not (Pawn|IsLocallyControlled (Reference|GetorCreatePlayer)))
      (CallFunction|S2CEquipmentItem _bsucceeded _equippedslot _itemstoragetype _itemequippedslottype _equippeditemuid))))

(event Custom|C2S_UnequipItem
  (params (TargetSlot :type E_EquipmentSlot%20Enum :default "NewEnumerator0") (TargetItemUID :type Guid%20Structure))
  ;[0.15 0.15 0.15 0.5] UnequipItem
  (bind (_bissucceeded _unequipslot _unequipitemuid) (Equipment|Action|TryUnequipItem TargetSlot TargetItemUID))
  (if _bissucceeded
    (Equipment|Visual|Action|HandleUpdateEquipmentVisual _unequipslot)
    (if (not (Pawn|IsLocallyControlled (Reference|GetorCreatePlayer)))
      (CallFunction|S2CUnEquipItem _unequipslot _unequipitemuid))))

(fn GetorCreatePlayer
  (Utilities|IsValid (Variables|Ref|GetPlayerRef)
    (:Is%20Valid
      _)
    (:Is%20Not%20Valid
      (bind _asbp_player (Utilities|Casting|CastToBP_Player (Components|GetOwner)))
      (Variables|Ref|SetPlayerRef _asbp_player)))
  (return (Variables|Ref|GetPlayerRef)))

(fn GetorCreateInventoryComponent
  (Utilities|IsValid (Variables|Ref|GetInventoryComponentRef)
    (:Is%20Valid
      _)
    (:Is%20Not%20Valid
      (Variables|Ref|SetInventoryComponentRef (Variables|/Game/InGame/Blueprints/Player/BP_Player.BP_Player_C|GetInventoryComponent (CallFunction|GetorCreatePlayer)))))
  (return (Variables|Ref|GetInventoryComponentRef)))

(fn InitializeEquipmnetVisualSlots
  (bind _playerref (Reference|GetorCreatePlayer))
  (Variables|Equipment|visual|SetEquipmentVisualSlots (Utilities|Map|MakeMap "NewEnumerator2" (Variables|/Game/InGame/Blueprints/Player/BP_Player.BP_Player_C|GetHelmetVisual _playerref) "NewEnumerator12" (Variables|/Game/InGame/Blueprints/Player/BP_Player.BP_Player_C|GetLeftWeaponVisual _playerref) "NewEnumerator13" (Variables|/Game/InGame/Blueprints/Player/BP_Player.BP_Player_C|GetRightWeaponVisual _playerref))))

(fn DropEquipmentItem
  (params (SlotType :type E_EquipmentSlot%20Enum :default "NewEnumerator0"))
  (bind _equipmentitems (Variables|Equipment|Data|GetEquipmentItems))
  (bind (_value _returnvalue) (Utilities|Map|Find _equipmentitems SlotType))
  (Utilities|FlowControl|Sequence
    (:then_0
      (LocalVariables|SetLocalUpdatedItemUID _value)
      (if (not _returnvalue)
        (return false)))
    (:then_1
      (bind _returnvalue_2 (Utilities|Map|Remove (Variables|Equipment|Data|GetEquipmentItems) SlotType))
      (if _returnvalue_2
        (if (Pawn|IsLocallyControlled (Reference|GetorCreatePlayer))
          (Equipment|Event|RefreshItem SlotType (Default|GetItembyUID (Reference|GetorCreateInventoryComponent) (LocalVariables|GetLocalUpdatedItemUID)))
          (return true)
          (else
            (return true)))
        (else
          (return false))))))

(fn TryEquipItem
  (params (TargetSlot :type E_EquipmentSlot%20Enum :default "NewEnumerator0") (StorageType :type E_StorageType%20Enum :default "NewEnumerator0") (EquippedSlotType :type E_EquipmentSlot%20Enum :default "NewEnumerator0") (TargetItemUID :type Guid%20Structure))
  (bind (_bexist _findslot) (Equipment|Internal|Query|FindCanEquipSlot TargetSlot TargetItemUID))
  (switch Utilities|FlowControl|Switch|SwitchonE_StorageType StorageType
    (:NewEnumerator0
      (LocalVariables|SetLocalTargetSlot _findslot)
      (if _bexist
        (bind _bsucceeded (Equipment|Internal|Action|SwapEquiptoInventoryItem (LocalVariables|GetLocalTargetSlot) (.ItemUID (Equipment|Query|GetEquipedItemUID (LocalVariables|GetLocalTargetSlot))) TargetItemUID))
        (return _bsucceeded TargetSlot StorageType EquippedSlotType TargetItemUID)
        (else
          (bind _bsucceeded_2 (Equipment|Internal|Action|EquiptoInventoryItem TargetSlot TargetItemUID))
          (return _bsucceeded_2 TargetSlot StorageType EquippedSlotType TargetItemUID))))
    (:NewEnumerator1
      (bind _bsucceeded_3 (Equipment|Internal|Action|SwapEquiptoEquipItem TargetSlot EquippedSlotType TargetItemUID))
      (return _bsucceeded_3 TargetSlot StorageType EquippedSlotType TargetItemUID))))

(fn AddEquipmentItem
  (params (Slot :type E_EquipmentSlot%20Enum :default "NewEnumerator0") (ItemUID :type Guid%20Structure))
  (Utilities|Map|Add (Variables|Equipment|Data|GetEquipmentItems) Slot ItemUID))

(fn RemoveEquipmentItem
  (params (TargetSlot :type E_EquipmentSlot%20Enum :default "NewEnumerator0"))
  (bind _returnvalue (Utilities|Map|Remove (Variables|Equipment|Data|GetEquipmentItems) TargetSlot))
  (return _returnvalue))

(fn EquiptoInventoryItem
  (params (TargetSlot :type E_EquipmentSlot%20Enum :default "NewEnumerator0") (TargetItemUID :type Guid%20Structure))
  (LocalVariables|SetLocalFindEquipSlot (.FindSlot (Equipment|Internal|Query|FindCanEquipSlot TargetSlot)))
  (bind _succeeded (Default|RemovetoInventory (Reference|GetorCreateInventoryComponent) TargetItemUID))
  (if _succeeded
    (Equipment|Internal|Update|AddEquipmentItem (LocalVariables|GetLocalFindEquipSlot) TargetItemUID)
    (Equipment|Event|RefreshItem (LocalVariables|GetLocalFindEquipSlot) (Default|GetItembyUID (Reference|GetorCreateInventoryComponent) TargetItemUID))
    (return true)
    (else
      (return false))))

(fn SwapEquiptoEquipItem
  (params (TargetSlot :type E_EquipmentSlot%20Enum :default "NewEnumerator0") (OriginSlot :type E_EquipmentSlot%20Enum :default "NewEnumerator0") (OriginItemUID :type Guid%20Structure))
  (bind _equipmentitems (Variables|Equipment|Data|GetEquipmentItems))
  (bind (_value _returnvalue) (Utilities|Map|Find _equipmentitems TargetSlot))
  (Utilities|FlowControl|Sequence
    (:then_0
      (if (Utilities|Enum|Equal(Enum) OriginSlot "NewEnumerator0")
        (return false)))
    (:then_1
      (LocalVariables|SetLocalTargetItemUID _value)
      (if _returnvalue
        (Equipment|Internal|Update|AddEquipmentItem TargetSlot OriginItemUID)
        (Equipment|Event|RefreshItem TargetSlot (Default|GetItembyUID (Reference|GetorCreateInventoryComponent) OriginItemUID))
        (Equipment|Internal|Update|AddEquipmentItem OriginSlot (LocalVariables|GetLocalTargetItemUID))
        (Equipment|Event|RefreshItem OriginSlot (Default|GetItembyUID (Reference|GetorCreateInventoryComponent) (LocalVariables|GetLocalTargetItemUID)))
        (return true)
        (else
          (Equipment|Internal|Update|RemoveEquipmentItem OriginSlot)
          (Equipment|Event|RefreshItem OriginSlot)
          (Equipment|Internal|Update|AddEquipmentItem TargetSlot OriginItemUID)
          (Equipment|Event|RefreshItem TargetSlot (Default|GetItembyUID (Reference|GetorCreateInventoryComponent) OriginItemUID))
          (return true))))))

(fn SwapEquiptoInventoryItem
  (params (EquippedSlot :type E_EquipmentSlot%20Enum :default "NewEnumerator0") (EquippedItemUID :type Guid%20Structure) (InventoryItemUID :type Guid%20Structure))
  (if (or (Utilities|Enum|Equal(Enum) EquippedSlot "NewEnumerator12") (Utilities|Enum|Equal(Enum) EquippedSlot "NewEnumerator13"))
    (bind _bsucceeded (Equipment|Internal|Action|SwapEquiptoInventoryWeapon InventoryItemUID EquippedSlot))
    (return _bsucceeded)
    (else
      (bind _succeeded (Default|RemovetoInventory (Reference|GetorCreateInventoryComponent) InventoryItemUID))
      (if _succeeded
        (bind _bsucceeded_2 (Default|TryAddEquipmentItem (Reference|GetorCreateInventoryComponent) EquippedItemUID))
        (if _bsucceeded_2
          (Equipment|Internal|Update|AddEquipmentItem EquippedSlot InventoryItemUID)
          (Equipment|Event|RefreshItem EquippedSlot (Default|GetItembyUID (Reference|GetorCreateInventoryComponent) InventoryItemUID))
          (return true)
          (else
            (Default|TryAddEquipmentItem (Reference|GetorCreateInventoryComponent) InventoryItemUID)
            (return false)))))))

(fn SwapEquiptoInventoryWeapon
  (params (InventoryItem :type Guid%20Structure) (TargetSlot :type E_EquipmentSlot%20Enum :default "NewEnumerator0"))
  (bind _equipmentitems (Variables|Equipment|Data|GetEquipmentItems))
  (bind _equipmentitems_2 (Variables|Equipment|Data|GetEquipmentItems))
  (bind (_value _returnvalue) (Utilities|Map|Find _equipmentitems_2 "NewEnumerator12"))
  (bind (_value_2 _returnvalue_2) (Utilities|Map|Find _equipmentitems "NewEnumerator13"))
  (bind (_bcanequip _bswapleftslot _bswaprightslot) (Equipment|Query|CanEquipWeaponstoInventory InventoryItem TargetSlot))
  (LocalVariables|SetbIsUpdateLeftWeapon _bswapleftslot)
  (LocalVariables|SetbIsUpdateRightWeapon _bswaprightslot)
  (if _bcanequip
    (Utilities|FlowControl|Sequence
      (:then_0
        (Default|RemovetoInventory (Reference|GetorCreateInventoryComponent) InventoryItem))
      (:then_1
        (if (LocalVariables|GetbIsUpdateLeftWeapon)
          (if _returnvalue
            (Default|TryAddEquipmentItem (Reference|GetorCreateInventoryComponent) _value)
            (Equipment|Internal|Update|RemoveEquipmentItem "NewEnumerator12"))))
      (:then_2
        (if (LocalVariables|GetbIsUpdateRightWeapon)
          (if _returnvalue_2
            (Default|TryAddEquipmentItem (Reference|GetorCreateInventoryComponent) _value_2)
            (Equipment|Internal|Update|RemoveEquipmentItem "NewEnumerator13"))))
      (:then_3
        (Equipment|Internal|Update|AddEquipmentItem TargetSlot InventoryItem)
        (Equipment|Event|RefreshItem TargetSlot (Default|GetItembyUID (Reference|GetorCreateInventoryComponent) InventoryItem))
        (return true)))))

(fn FindCanEquipSlot
  (params (SlotType :type E_EquipmentSlot%20Enum :default "NewEnumerator0") (TargetItemUID :type Guid%20Structure))
  (bind _equipmentitems (Variables|Equipment|Data|GetEquipmentItems))
  (bind (_value _returnvalue) (Utilities|Map|Find _equipmentitems "NewEnumerator12"))
  (if (Utilities|Enum|Equal(Enum) SlotType "NewEnumerator10")
    (Utilities|FlowControl|Sequence
      (:then_0
        (if (not (.ReturnValue (Utilities|Map|Find (Variables|Equipment|Data|GetEquipmentItems) "NewEnumerator6")))
          (return false "NewEnumerator6")))
      (:then_1
        (if (.ReturnValue (Utilities|Map|Find (Variables|Equipment|Data|GetEquipmentItems) "NewEnumerator7"))
          (return true "NewEnumerator6")
          (else
            (return false "NewEnumerator7")))))
    (elif (Math|Boolean|ORBoolean (Utilities|Enum|Equal(Enum) SlotType "NewEnumerator1") (Utilities|Enum|Equal(Enum) SlotType "NewEnumerator12") (Utilities|Enum|Equal(Enum) SlotType "NewEnumerator13"))
      ;[0.15 0.15 0.15 0.5] 현재 장착하고 싶은 무기 : 양손?
      (if (Equipment|Query|IsTwoHandedItem (Default|GetItembyUID (Reference|GetorCreateInventoryComponent) TargetItemUID))
        (return (not (and (not (.ReturnValue (Utilities|Map|Find (Variables|Equipment|Data|GetEquipmentItems) "NewEnumerator12"))) (not (.ReturnValue (Utilities|Map|Find (Variables|Equipment|Data|GetEquipmentItems) "NewEnumerator13"))))) "NewEnumerator12")
        (else
          ;[0.15 0.15 0.15 0.5] 한손 무기 장착 가능?
          (Utilities|FlowControl|Sequence
            (:then_0
              (if _returnvalue
                (if (Equipment|Query|IsTwoHandedItem (Default|GetItembyUID (Reference|GetorCreateInventoryComponent) _value))
                  (return true "NewEnumerator12"))
                (else
                  (return false "NewEnumerator12"))))
            (:then_1
              (if (.ReturnValue (Utilities|Map|Find (Variables|Equipment|Data|GetEquipmentItems) "NewEnumerator13"))
                (if (Utilities|Enum|Equal(Enum) SlotType "NewEnumerator13")
                  (return true "NewEnumerator13")
                  (else
                    (return true "NewEnumerator12")))
                (else
                  (return false "NewEnumerator13")))))))
      (else
        (return (Utilities|Map|Contains (Variables|Equipment|Data|GetEquipmentItems) SlotType) SlotType)))))

(fn CanReplacetoInventoryItem
  (params (TargetSlot :type E_EquipmentSlot%20Enum :default "NewEnumerator0") (TargetItemUID :type Guid%20Structure))
  (bind (_itemuid _bsuceeded) (Equipment|Query|GetEquipedItemUID TargetSlot))
  (LocalVariables|SetLocalEquippedItem _itemuid)
  (if _bsuceeded
    (bind (_bcanstore _startpoint) (Default|FindFirstAvailableSlot :self (Reference|GetorCreateInventoryComponent) :TargetItemUID (LocalVariables|GetLocalEquippedItem) :IgnoreItemUID TargetItemUID))
    (if _bcanstore
      (return true _startpoint (LocalVariables|GetLocalEquippedItem))
      (else
        (return false "" "")))
    (else
      (return false (LocalVariables|GetLocalFalseResult) ""))))

(fn CanEquipItem
  (params (TargetSlot :type E_EquipmentSlot%20Enum :default "NewEnumerator0") (TargetItemUID :type Guid%20Structure))
  (bind (_bexist _findslot) (Equipment|Internal|Query|FindCanEquipSlot TargetSlot))
  (Utilities|FlowControl|Sequence
    (:then_0
      (LocalVariables|SetLocalTargetSlot _findslot)
      (if (not _bexist)
        (return false "NewEnumerator0" "")))
    (:then_1
      (return (not (.ReturnValue (Utilities|Map|Find (Variables|Equipment|Data|GetEquipmentItems) (LocalVariables|GetLocalTargetSlot)))) (LocalVariables|GetLocalTargetSlot) (.Value (Utilities|Map|Find (Variables|Equipment|Data|GetEquipmentItems) (LocalVariables|GetLocalTargetSlot)))))))

(fn GetEquipedItemUID
  (params (Slot :type E_EquipmentSlot%20Enum :default "NewEnumerator0"))
  (bind _equipmentitems (Variables|Equipment|Data|GetEquipmentItems))
  (bind (_value _returnvalue) (Utilities|Map|Find _equipmentitems Slot))
  (return _value _returnvalue))

(fn IsTwoHandedItem
  (params (TargetItem :type ST%20Item%20Instance%20Structure))
  (bind _itemdefinition (Utilities|Struct|BreakST_ItemInstance TargetItem))
  (Utilities|IsValid _itemdefinition
    (:Is%20Valid
      (bind _aspda_equipment_definition (Utilities|Casting|CastToPDA_EquipmentDefinition _itemdefinition))
      (return (Variables|/Game/InGame/Datas/PDA/Item/PDA_EquipmentDefinition.PDA_EquipmentDefinition_C|GetbIsTwoHanded _aspda_equipment_definition)))
    (:Is%20Not%20Valid
      (return false))))

(fn CanEquipWeaponstoInventory
  (params (IgnoreItemUID :type Guid%20Structure) (TargetSlot :type E_EquipmentSlot%20Enum :default "NewEnumerator0"))
  (Utilities|FlowControl|Sequence
    (:then_1
      (if (Equipment|Query|IsTwoHandedItem (Default|GetItembyUID (Reference|GetorCreateInventoryComponent) IgnoreItemUID))
        (bind (_bcanplace _bcanplaceleft _bcanplaceright) (Default|CanPlaceWeapon (Reference|GetorCreateInventoryComponent) (.Value (Utilities|Map|Find (Variables|Equipment|Data|GetEquipmentItems) "NewEnumerator12")) (.Value (Utilities|Map|Find (Variables|Equipment|Data|GetEquipmentItems) "NewEnumerator13")) IgnoreItemUID))
        (return _bcanplace _bcanplaceleft _bcanplaceright)
        (elif (Utilities|Enum|Equal(Enum) TargetSlot "NewEnumerator12")
          (bind (_bcanplace_2 _bcanplaceleft_2 _bcanplaceright_2) (Default|CanPlaceWeapon :self (Reference|GetorCreateInventoryComponent) :LeftItemUID (.Value (Utilities|Map|Find (Variables|Equipment|Data|GetEquipmentItems) "NewEnumerator12")) :IgnoreItemUID IgnoreItemUID))
          (return _bcanplace_2 _bcanplaceleft_2 _bcanplaceright_2)
          (else
            (bind (_bcanplace_3 _bcanplaceleft_3 _bcanplaceright_3) (Default|CanPlaceWeapon :self (Reference|GetorCreateInventoryComponent) :RightItemUID (.Value (Utilities|Map|Find (Variables|Equipment|Data|GetEquipmentItems) "NewEnumerator13")) :IgnoreItemUID IgnoreItemUID))
            (return _bcanplace_3 _bcanplaceleft_3 _bcanplaceright_3)))))))

(fn RefreshItem
  (params (ChangedSlot :type E_EquipmentSlot%20Enum :default "NewEnumerator0") (EquipmentItem :type ST%20Item%20Instance%20Structure))
  (if (Pawn|IsLocallyControlled (Reference|GetorCreatePlayer))
    (Default|CallOnEquipmentChanged ChangedSlot EquipmentItem)))

(fn TryUnequipItem
  (params (TargetSlot :type E_EquipmentSlot%20Enum :default "NewEnumerator0") (TargetItemUID :type Guid%20Structure))
  (Equipment|Internal|Update|RemoveEquipmentItem TargetSlot)
  (bind _bsucceeded (Default|TryAddEquipmentItem (Reference|GetorCreateInventoryComponent) TargetItemUID))
  (if _bsucceeded
    (Equipment|Event|RefreshItem TargetSlot)
    (return true TargetSlot TargetItemUID)
    (else
      (Equipment|Internal|Update|AddEquipmentItem TargetSlot TargetItemUID)
      (return false "NewEnumerator0" ""))))

(fn HandleUpdateEquipmentVisual
  (params (UpdatedSlot :type E_EquipmentSlot%20Enum :default "NewEnumerator0"))
  (switch Utilities|FlowControl|Switch|SwitchonE_EquipmentSlot UpdatedSlot
    (:NewEnumerator0
      _)
    (:NewEnumerator1
      (bind _weaponbehaviorstate (Equipment|Visual|Internal|UpdateWeaponVisual :!label _label))
      (Variables|Equipment|Data|SetCurrentWeaponBehaviorState _weaponbehaviorstate)
      (return true))
    (:NewEnumerator13
      (goto _label))
    (:NewEnumerator12
      (goto _label))
    (:NewEnumerator2
      (Equipment|Visual|Internal|UpdateArmorVisual UpdatedSlot)
      (return true))
    (:NewEnumerator4
      _)
    (:NewEnumerator5
      _)
    (:NewEnumerator10
      _)
    (:NewEnumerator6
      _)
    (:NewEnumerator7
      _)
    (:NewEnumerator8
      _)
    (:NewEnumerator9
      _))
  (return false))

(fn GetCurrentWeaponBehaviorState
  (Utilities|FlowControl|Sequence
    (:then_0
      (bind _output_get (LocalVariables|SetLocalLeftWeaponUID (.Value (Utilities|Map|Find (Variables|Equipment|Data|GetEquipmentItems) "NewEnumerator12"))))
      (if (Guid|IsValidGuid _output_get)
        (LocalVariables|SetLocalReturnType "NewEnumerator0")
        (Math|Integer|IncrementInt (LocalVariables|GetLocalWeaponCount))))
    (:then_1
      (if (.ReturnValue (Utilities|Map|Find (Variables|Equipment|Data|GetEquipmentItems) "NewEnumerator13"))
        (LocalVariables|SetLocalReturnType "NewEnumerator5")
        (Math|Integer|IncrementInt (LocalVariables|GetLocalWeaponCount))))
    (:then_2
      (if (Equipment|Query|IsTwoHandedItem (Default|GetItembyUID (Reference|GetorCreateInventoryComponent) (LocalVariables|GetLocalLeftWeaponUID)))
        (LocalVariables|SetLocalReturnType "NewEnumerator1")))
    (:then_3
      (return (LocalVariables|GetLocalReturnType) (|({E591B4F3-44D2-1358-AC44-718CBF174758}>=2))))))

(fn UpdateWeaponVisual
  (bind (_currentweaponbehaviorstate _bisdual) (Equipment|Visual|Query|GetCurrentWeaponBehaviorState))
  (bind _equipmentvisualslots (Variables|Equipment|visual|GetEquipmentVisualSlots))
  (bind _equipmentvisualslots_2 (Variables|Equipment|visual|GetEquipmentVisualSlots))
  (bind (_value _returnvalue) (Utilities|Map|Find _equipmentvisualslots "NewEnumerator13"))
  (bind (_value_2 _returnvalue_2) (Utilities|Map|Find _equipmentvisualslots_2 "NewEnumerator12"))
  (Utilities|FlowControl|Sequence
    (:then_0
      (LocalVariables|SetLocalCurrentWeaponBehaviorState _currentweaponbehaviorstate)
      (LocalVariables|SetbLocalCurrentDualWeaponEquip _bisdual))
    (:then_1
      (switch Utilities|FlowControl|Switch|SwitchonE_WeaponBehaviorType (LocalVariables|GetLocalCurrentWeaponBehaviorState)
        (:NewEnumerator4
          (bind _output_get (LocalVariables|SetLocalUpdatedLeftStaticMesh 0))
          (LocalVariables|SetLocalUpdatedRightStaticMesh _output_get))
        (:NewEnumerator0
          (bind _equipmentstaticmesh (CallFunction|GetEquipmentStaticMeshbyUID "NewEnumerator12"))
          (LocalVariables|SetLocalUpdatedLeftStaticMesh _equipmentstaticmesh)
          (LocalVariables|SetLocalUpdatedRightStaticMesh 0))
        (:NewEnumerator1
          (bind _equipmentstaticmesh_2 (CallFunction|GetEquipmentStaticMeshbyUID "NewEnumerator12"))
          (LocalVariables|SetLocalUpdatedLeftStaticMesh _equipmentstaticmesh_2)
          (LocalVariables|SetLocalUpdatedRightStaticMesh 0))
        (:NewEnumerator5
          (bind _equipmentstaticmesh_3 (CallFunction|GetEquipmentStaticMeshbyUID "NewEnumerator12"))
          (LocalVariables|SetLocalUpdatedLeftStaticMesh _equipmentstaticmesh_3)
          (bind _equipmentstaticmesh_4 (CallFunction|GetEquipmentStaticMeshbyUID "NewEnumerator13"))
          (LocalVariables|SetLocalUpdatedRightStaticMesh _equipmentstaticmesh_4))))
    (:then_2
      (if _returnvalue_2
        (Components|StaticMesh|SetStaticMesh _value_2 (LocalVariables|GetLocalUpdatedLeftStaticMesh))))
    (:then_3
      (if _returnvalue
        (Components|StaticMesh|SetStaticMesh _value (LocalVariables|GetLocalUpdatedRightStaticMesh))))
    (:then_4
      (return (LocalVariables|GetLocalCurrentWeaponBehaviorState)))))

(fn UpdateArmorVisual
  (params (UpdatedSlot :type E_EquipmentSlot%20Enum :default "NewEnumerator0"))
  (Utilities|FlowControl|Sequence
    (:then_0
      (LocalVariables|SetLocalCurrentItemUID (.Value (Utilities|Map|Find (Variables|Equipment|Data|GetEquipmentItems) UpdatedSlot))))
    (:then_1
      (LocalVariables|SetLocalCurrentEquipmentVisual (.Value (Utilities|Map|Find (Variables|Equipment|visual|GetEquipmentVisualSlots) UpdatedSlot))))
    (:then_2
      (if (Guid|IsValidGuid (LocalVariables|GetLocalCurrentItemUID))
        (bind _aspda_equipment_definition (Utilities|Casting|CastToPDA_EquipmentDefinition (Utilities|Struct|BreakST_ItemInstance (Default|GetItembyUID (Reference|GetorCreateInventoryComponent) (LocalVariables|GetLocalCurrentItemUID)))))
        (Variables|Equipment|Data|SetCurrentWeaponBehavior (Variables|/Game/InGame/Datas/PDA/Item/PDA_EquipmentDefinition.PDA_EquipmentDefinition_C|GetWeaponBehavior _aspda_equipment_definition))
        (Components|StaticMesh|SetStaticMesh (LocalVariables|GetLocalCurrentEquipmentVisual) (Variables|/Game/InGame/Datas/PDA/Item/PDA_EquipmentDefinition.PDA_EquipmentDefinition_C|GetEquipmentStaticMesh _aspda_equipment_definition))
        (else
          (Components|StaticMesh|SetStaticMesh (LocalVariables|GetLocalCurrentEquipmentVisual) 0))))))

(fn GetEquipmentStaticMeshbyUID
  (params (EquipmentSlot :type E_EquipmentSlot%20Enum :default "NewEnumerator0"))
  (bind _aspda_equipment_definition (Utilities|Casting|CastToPDA_EquipmentDefinition (Utilities|Struct|BreakST_ItemInstance (Default|GetItembyUID (Variables|Ref|GetInventoryComponentRef) (.Value (Utilities|Map|Find (Variables|Equipment|Data|GetEquipmentItems) EquipmentSlot))))))
  (return (Variables|/Game/InGame/Datas/PDA/Item/PDA_EquipmentDefinition.PDA_EquipmentDefinition_C|GetEquipmentStaticMesh _aspda_equipment_definition)))