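; Monster character Blueprint that switches between normal and combat movement speed and plays melee-style attack montages.
; S2M events start or stop chase and trigger Attack, which disables further attacks, plays a random montage section and sets a timer.
; Tick draws debug sphere traces and a forward fan of line traces without using their results.
; Damage processing queries MonsterStatComponent for death (passing zero, not AppliedDamage) and stops the attack animation when dead.
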(event EventBeginPlay
  (|CallParentFunction) ; This node is disabled and will not be called.\nDrag off pins to build functionality.
)

(event Collision|EventActorBeginOverlap
  (params (OtherActor :type Actor%20Object%20Reference))
  (|CallParentFunction OtherActor) ; This node is disabled and will not be called.\nDrag off pins to build functionality.
)

(event EventTick
  (params (DeltaSeconds :type Float%20%28single-precision%29))
  (bind _returnvalue (Transformation|GetActorLocation))
  (bind _returnvalue_2 (Transformation|GetActorLocation))
  (bind _returnvalue_3 (Transformation|GetActorLocation))
  (|CallParentFunction DeltaSeconds)
  (Collision|SphereTraceByChannel _returnvalue_2 _returnvalue_2 3e+02 "TraceTypeQuery1" false 0 "ForDuration" true "(R=1.000000,G=0.000000,B=0.000000,A=1.000000)" "(R=0.000000,G=1.000000,B=0.000000,A=1.000000)" 0.0)
  (Collision|SphereTraceByChannel _returnvalue_3 _returnvalue_3 1.2e+03 "TraceTypeQuery1" false 0 "ForDuration" true "(R=1.000000,G=0.000000,B=0.969961,A=1.000000)" "(R=0.320997,G=0.437344,B=1.000000,A=1.000000)" 0.0)
  (for _index (range 0 4)
    (Collision|MultiLineTraceByChannel _returnvalue (+ _returnvalue (* (Math|Vector|RotateVectorAroundAxis (Transformation|GetActorForwardVector) (|((Index*22.500000)-45.000000) _index) "0.000000,0.000000,1.000000") 3e+03)) "TraceTypeQuery1" false 0 "ForDuration" true "(R=1.000000,G=0.000000,B=0.000000,A=1.000000)" "(R=0.000000,G=1.000000,B=0.000000,A=1.000000)" 0.0)))

(event Game|Damage|EventPointDamage
  (params (Damage :type Float%20%28single-precision%29) (DamageType :type Damage%20Type%20Object%20Reference) (HitLocation :type Vector :default "0, 0, 0") (HitNormal :type Vector :default "0, 0, 0") (HitComponent :type Primitive%20Component%20Object%20Reference) (BoneName :type Name :default "None") (ShotFromDirection :type Vector :default "0, 0, 0") (InstigatedBy :type Controller%20Object%20Reference) (DamageCauser :type Actor%20Object%20Reference) (HitInfo :type Hit%20Result%20Structure%20%28by%20ref%29))
  (|CallParentFunction Damage DamageType HitLocation HitNormal HitComponent BoneName ShotFromDirection InstigatedBy DamageCauser HitInfo))

(event Custom|S2M_StopChase
  (CallFunction|ChangeCombatModeSpeed false))

(event Custom|S2M_PlayAttack
  (CallFunction|Attack))

(event Custom|S2M_StopAttackAnim
  (bind _mesh (Variables|Character|GetMesh))
  (bind _returnvalue (Components|SkeletalMesh|GetAnimInstance _mesh))
  (Utilities|IsValid _returnvalue
    (:Is%20Valid
      (Animation|Montage|MontageStop _returnvalue 0.0 "/Game/Assets/Monster/Animations/AM_Attack.AM_Attack"))))

(event Custom|S2M_StartChase
  (CallFunction|ChangeCombatModeSpeed true))

(fn ConstructionScript
  (|CallParentFunction))

(fn Attack
  (Variables|Default|SetbIsEnableAttack false)
  (CallFunction|ChangeCombatModeSpeed true)
  (Animation|PlayAnimMontage "/Game/Assets/Monster/Animations/AM_Attack.AM_Attack" 1.0 (Utilities|String|StringToName (Utilities|String|Append "Attack_" (Utilities|String|ToString(Integer) (Math|Random|RandomInteger 2)))))
  (Utilities|Time|SetTimerbyEvent (EventDispatchers|CreateEvent :!event EnableAttack) 2.0)
  (return 0.0))

(fn ChangeCombatModeSpeed
  (params (CombatMode :type Boolean))
  (bind _charactermovement (Variables|Character|GetCharacterMovement))
  (if CombatMode
    (Variables|Default|SetbIsCombat true)
    (Variables|/Script/Engine.CharacterMovementComponent|SetMaxWalkSpeed _charactermovement 5.5e+02)
    (else
      (Variables|Default|SetbIsCombat false)
      (Variables|/Script/Engine.CharacterMovementComponent|SetMaxWalkSpeed _charactermovement 3e+02))))

(fn TakeDamageProcess
  (params (AppliedDamage :type Float%20%28double-precision%29))
  (|CallParentFunction AppliedDamage)
  (bind _bisdead (Default|TakeDamage (Variables|Default|GetMonsterStatComponent) 0.0))
  (bind _output_get (Variables|Default|SetbIsDead _bisdead))
  (if _output_get
    (CallFunction|S2MStopAttackAnim)))