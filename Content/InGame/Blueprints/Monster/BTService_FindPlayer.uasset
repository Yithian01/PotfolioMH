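; Behavior tree service for monster AI that detects the player by proximity.
; On activation it finds the BP_Player actor and caches the reference if none is valid.
; Each tick it writes that player to the PlayerObject blackboard key when within FindDistance of the owner, and clears the key otherwise.
; Detection uses straight-line distance only, with no line-of-sight check.
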(event `self.ReceiveActivationAI`
  (params (OwnerController :type "AIController Object Reference") (ControlledPawn :type "Pawn Object Reference"))
  (`/Engine/EditorBlueprintResources/StandardMacros.IsValid` (`self.PlayerRef`)
    (:`Is Not Valid`
      (bind _returnvalue (`GameplayStatics.GetActorOfClass` "/Game/InGame/Blueprints/Player/BP_Player.BP_Player_C"))
      (set `self.PlayerRef` _returnvalue))))

(event `self.ReceiveTick`
  (params (OwnerActor :type "Actor Object Reference") (DeltaSeconds :type "Float (single-precision)"))
  (if (<= (`KismetMathLibrary.Vector_Distance` (`Actor.K2_GetActorLocation` (`self.PlayerRef`)) (`Actor.K2_GetActorLocation` OwnerActor)) (`self.FindDistance`))
    (`BTFunctionLibrary.SetBlackboardValueAsObject` (`self.PlayerObject`) (`self.PlayerRef`))
    (else
      (`BTFunctionLibrary.SetBlackboardValueAsObject` (`self.PlayerObject`)))))