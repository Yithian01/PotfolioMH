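; Drag-and-drop operation for dragging an item in the inventory UI.
; On drag cancel, it notifies the source widget and then, if valid, the inventory panel, both only while the source is valid.
; GetTopLeftOffset returns half the source widget's desired size as an integer point, or reports failure without a source.
; The inventory and equipment cancel functions are empty stubs.
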(event `self.DragCancelled`
  (params (PointerEvent :type "PointerEvent Structure (by ref)"))
  (`/Engine/EditorBlueprintResources/StandardMacros.IsValid` (`self.SourceUI`)
    (:`Is Valid`
      (message `/Game/InGame/Blueprints/Item/BPI_InventoryItemDrag.HandleDragCancelled` (`self.SourceUI`))
      (`/Engine/EditorBlueprintResources/StandardMacros.IsValid` (`self.InventoryPanelUI`)
        (:`Is Valid`
          (message `/Game/InGame/Blueprints/Item/BPI_InventoryItemDrag.HandleDragCancelled` (`self.InventoryPanelUI`)))))))

(fn `GetTopLeftOffset`
  (returns (bSucceeded :type Boolean) (UISize :type "IntPoint Structure"))
  (`/Engine/EditorBlueprintResources/StandardMacros.IsValid` (`self.SourceUI`)
    (:`Is Valid`
      (return true (`KismetMathLibrary.Conv_Vector2DToIntPoint` (/ (`Widget.GetDesiredSize` (`self.SourceUI`)) (2.0 2.0)))))
    (:`Is Not Valid`
      (return false))))

(fn `OnCancelledEquipmentUI`)

(fn `OnCancelledInventoryUI`)