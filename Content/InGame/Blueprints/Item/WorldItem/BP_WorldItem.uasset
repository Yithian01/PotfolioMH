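; BP_WorldItem is the world actor for an item instance that can be dropped and picked up.
; Its body takes mesh and rotation from the item definition at construction, and can be highlighted through custom depth.
; Pickup runs only on the server, handing the instance to the target inventory and destroying the actor on success.
; Dropping enables physics with an impulse, then the body reverts to query-only collision without simulation once it sleeps.
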(event `self.Body.OnComponentSleep`
  (params (SleepingComponent :type "PrimitiveComponent Object Reference") (BoneName :type Name))
  (`PrimitiveComponent.SetSimulatePhysics` SleepingComponent false)
  (`PrimitiveComponent.SetCollisionEnabled` SleepingComponent "QueryOnly"))

(fn `RefreshWorldItemVisual`
  (bind (_iteminstance_itemuid _iteminstance_itemdefinition) (break `/Game/InGame/Datas/Struct/Item/ST_ItemInstance` (`self.ItemInstance`)))
  (`/Engine/EditorBlueprintResources/StandardMacros.IsValid` _iteminstance_itemdefinition
    (:`Is Valid`
      (`StaticMeshComponent.SetStaticMesh` (`self.Body`) (`/Game/InGame/Datas/PDA/Item/PDA_ItemDefinition.WorldItemStaticMesh` _iteminstance_itemdefinition))
      (`SceneComponent.K2_SetWorldRotation` (`self.Body`) (`/Game/InGame/Datas/PDA/Item/PDA_ItemDefinition.WorldRotationOffset` _iteminstance_itemdefinition) false false))))

(fn `SetPickupHighlight`
  (params (bIsHighlight :type Boolean))
  (`PrimitiveComponent.SetRenderCustomDepth` (`self.Body`) bIsHighlight))

(fn `StartDropPhysics`
  (params (DropLocation :type "Vector Structure"))
  (`PrimitiveComponent.SetCollisionEnabled` (`self.Body`) "QueryAndPhysics")
  (`PrimitiveComponent.SetSimulatePhysics` (`self.Body`) true)
  (`PrimitiveComponent.SetMassScale` (`self.Body`) "None" 500.0)
  (`PrimitiveComponent.AddImpulse` (`self.Body`) (+ (* (`local.DropLocation`) 120.0) (`KismetMathLibrary.MakeVector` 0.0 0.0 60.0)) "None" false))

(fn `TryPickupItem`
  (params (TargetInventoryRef :type "/Game/InGame/Blueprints/Components/BPC_InventoryComponent Object Reference") (TargetEquipmentRef :type "/Game/InGame/Blueprints/Components/BPC_EquipmentComponent Object Reference"))
  (returns (bSucceded :type Boolean) (AddedItem :type "/Game/InGame/Datas/Struct/Item/ST_ItemInstance Structure"))
  (if (`KismetSystemLibrary.IsServer`)
    (`/Engine/EditorBlueprintResources/StandardMacros.IsValid` (`.ItemDefinition_9_88C99C9B4588673D38DD769AFBFB6841` (break `/Game/InGame/Datas/Struct/Item/ST_ItemInstance` (`self.ItemInstance`)))
      (:`Is Valid`
        (`/Engine/EditorBlueprintResources/StandardMacros.IsValid` (`local.TargetInventoryRef`)
          (:`Is Valid`
            (bind _succeeded_ (`/Game/InGame/Blueprints/Components/BPC_InventoryComponent.PickupItem` :`self` (`local.TargetInventoryRef`) :`NewItem` (`self.ItemInstance`)))
            (if _succeeded_
              (`self.K2_DestroyActor`)
              (return true (`self.ItemInstance`))
              (else
                (return false (`self.ItemInstance`)))))
          (:`Is Not Valid`
            (return false (`self.ItemInstance`)))))
      (:`Is Not Valid`
        (return false (`self.ItemInstance`))))))

(fn `UserConstructionScript`
  (`self.RefreshWorldItemVisual`))