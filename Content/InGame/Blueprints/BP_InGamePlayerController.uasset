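; In-game player controller that manages the local player's UI, input mode and Enhanced Input mapping.
; Widgets are created lazily by type and cached in a registry; requests toggle one active widget at a time, which drives cursor visibility and input mode.
; Boss changes from the game state are bound to the main HUD widget.
; S2C_ShowBloodScreen plays the blood-screen effect.
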(event `self.ReceiveBeginPlay`
  (if (`self.IsLocalPlayerController` self)
    ; InLocal
    (`|ExecutionSequence`
      (:`then_0`
        (`self.InitializeRef`)
        (`self.InitalizeInGameUI`))
      (:`then_1`
        (add `/Game/InGame/Blueprints/BP_InGameGameState.OnBossChanged` (`self.GameStateRef`) (delegate `HandleBossChanged`))
        (`/Game/InGame/Blueprints/BP_InGameGameState.RefreshBossMonsterRef` (`self.GameStateRef`)))
      (:`then_2`
        (`self.UpdateInputMode`))
      (:`then_3`
        (`EnhancedInputSubsystemInterface.AddMappingContext` (subsystem `EnhancedInputLocalPlayerSubsystem`) "/Game/InGame/Input/IMC_InGame.IMC_InGame" 0 (struct))))))

(event `HandleBossChanged`
  (params (BossMonster :type "/Game/InGame/Blueprints/Monster/BP_Monster Object Reference"))
  ; InLocal
  (`/Engine/EditorBlueprintResources/StandardMacros.IsValid` BossMonster
    (:`Is Valid`
      (bind _ui (`self.GetOrCreateUI` "NewEnumerator2"))
      (bind _aswbp_in_game_main (cast `/Game/UI/InGame/WBP_InGameMain` _ui))
      (`/Game/UI/InGame/WBP_InGameMain.HandleBossMonsterBind` _aswbp_in_game_main BossMonster))))

(event `S2C_ShowBloodScreen`
  (bind _ui (`self.GetOrCreateUI` "NewEnumerator4"))
  (bind _aswbp_blood_screen (cast `/Game/UI/InGame/Effect/WBP_BloodScreen` _ui))
  (`/Game/UI/InGame/Effect/WBP_BloodScreen.PlayBloodEffect` _aswbp_blood_screen))

(fn `CloseUI`
  (`Widget.SetVisibility` (`self.ActiveUI`) "Collapsed")
  (set `self.ActiveUI` null))

(fn `GetOrCreatePlayerRef`
  (returns (PlayerRef :type "/Game/InGame/Blueprints/Player/BP_Player Object Reference"))
  (`/Engine/EditorBlueprintResources/StandardMacros.IsValid` (`self.PlayerRef`)
    (:`Is Valid`
      _)
    (:`Is Not Valid`
      (bind _asbp_player (cast `/Game/InGame/Blueprints/Player/BP_Player` (`self.K2_GetPawn`)))
      (set `self.PlayerRef` _asbp_player)))
  (return (`self.PlayerRef`)))

(fn `GetOrCreateUI`
  (params (UIType :type "/Game/InGame/Datas/Enum/UI/E_UIType Enum" :default "NewEnumerator0"))
  (returns (UI :type "UserWidget Object Reference"))
  (locals (LocalTargetUI :type "UserWidget Object Reference"))
  (bind _output_get (set `local.LocalTargetUI` (`BlueprintMapLibrary.Map_Find` (`self.UIRegistory`) UIType)))
  (`/Engine/EditorBlueprintResources/StandardMacros.IsValid` _output_get
    (:`Is Valid`
      (return (`local.LocalTargetUI`)))
    (:`Is Not Valid`
      (bind _returnvalue (`|CreateWidget` (select `/Game/InGame/Datas/Enum/UI/E_UIType` (`local.UIType`) :`NewEnumerator0` "/Game/UI/InGame/Inventory/WBP_Inventory.WBP_Inventory_C" :`NewEnumerator2` "/Game/UI/InGame/WBP_InGameMain.WBP_InGameMain_C" :`NewEnumerator4` "/Game/UI/InGame/Effect/WBP_BloodScreen.WBP_BloodScreen_C" :!type "UserWidget Class Reference") self))
      (bind _output_get_2 (set `local.LocalTargetUI` _returnvalue))
      (`UserWidget.AddToViewport` _output_get_2 0)
      (`BlueprintMapLibrary.Map_Add` (`self.UIRegistory`) (`local.UIType`) (`local.LocalTargetUI`))
      (return (`local.LocalTargetUI`)))))

(fn `InitalizeInGameUI`
  (`self.GetOrCreateUI` "NewEnumerator2"))

(fn `InitializeRef`
  (bind _asbp_in_game_game_state (cast `/Game/InGame/Blueprints/BP_InGameGameState` (`GameplayStatics.GetGameState`)))
  (set `self.GameStateRef` _asbp_in_game_game_state))

(fn `OpenUI`
  (params (TargetUI :type "UserWidget Object Reference"))
  (`|ExecutionSequence`
    (:`then_0`
      (`/Engine/EditorBlueprintResources/StandardMacros.IsValid` (`self.ActiveUI`)
        (:`Is Valid`
          (`self.CloseUI`))))
    (:`then_1`
      (`Widget.SetVisibility` (`local.TargetUI`) "Visible")
      (set `self.ActiveUI` (`local.TargetUI`)))))

(fn `ProcessRequestUI`
  (params (UIType :type "/Game/InGame/Datas/Enum/UI/E_UIType Enum" :default "NewEnumerator0"))
  (locals (LocalTargetUI :type "UserWidget Object Reference"))
  (`|ExecutionSequence`
    (:`then_0`
      (bind _ui (`self.GetOrCreateUI` UIType))
      (if (== _ui (`self.ActiveUI`))
        (`self.CloseUI`)
        (else
          (`self.OpenUI` _ui))))
    (:`then_1`
      (`self.UpdateInputMode`))))

(fn `RequestUI`
  (params (UIType :type "/Game/InGame/Datas/Enum/UI/E_UIType Enum" :default "NewEnumerator0"))
  (`self.ProcessRequestUI` UIType))

(fn `UpdateInputMode`
  (bind _output_get (set `self.bShowMouseCursor` (`KismetSystemLibrary.IsValid` (`self.ActiveUI`))))
  (if _output_get
    (`WidgetBlueprintLibrary.SetInputMode_GameAndUIEx` self null "DoNotLock" false)
    (else
      (`WidgetBlueprintLibrary.SetInputMode_GameOnly` self))))

(fn `UserConstructionScript`)