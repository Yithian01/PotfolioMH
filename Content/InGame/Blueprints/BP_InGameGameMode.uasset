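; BP_InGameGameMode is the in-game game mode that spawns the boss monster and world item drops.
; On BeginPlay it caches the in-game GameState, spawns a BP_Monster at the boss spawn point, and registers it with the GameState.
; SpawnItem creates a BP_WorldItem from an item instance, scaled by its definition's size offset, starts drop physics with an impulse direction, and reports success.
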(event `self.ReceiveBeginPlay`
  (`self.Initialize`)
  (`self.BossSpawn`)
  (`/Game/InGame/Blueprints/BP_InGameGameState.SetBossMonster` (`self.GameStateRef`) (`self.BossRef`)))

(fn `BossSpawn`
  (bind _returnvalue (`|SpawnActorFromClass` "/Game/InGame/Blueprints/Monster/BP_Monster.BP_Monster_C" (`self.BossSpawnPoint`) "AdjustIfPossibleButAlwaysSpawn" "MultiplyWithRoot" null null))
  (set `self.BossRef` _returnvalue))

(fn `Initialize`
  (bind _asbp_in_game_game_state (cast `/Game/InGame/Blueprints/BP_InGameGameState` (`GameplayStatics.GetGameState`)))
  (set `self.GameStateRef` _asbp_in_game_game_state))

(fn `SpawnItem`
  (params (SpawnItem :type "/Game/InGame/Datas/Struct/Item/ST_ItemInstance Structure") (DropLocation :type "Transform Structure") (ImpluseDirection :type "Vector Structure"))
  (returns (bSuccessded :type Boolean))
  (bind (_spawnitem_itemuid _spawnitem_itemdefinition) (break `/Game/InGame/Datas/Struct/Item/ST_ItemInstance` (`local.SpawnItem`)))
  (bind (_droplocation_location _droplocation_rotation) (`KismetMathLibrary.BreakTransform` (`local.DropLocation`)))
  (bind _returnvalue (`|SpawnActorFromClass` "/Game/InGame/Blueprints/Item/WorldItem/BP_WorldItem.BP_WorldItem_C" (`KismetMathLibrary.MakeTransform` _droplocation_location _droplocation_rotation (`/Game/InGame/Datas/PDA/Item/PDA_ItemDefinition.SizeOffset` _spawnitem_itemdefinition)) "AdjustIfPossibleButAlwaysSpawn" "MultiplyWithRoot" null (`local.SpawnItem`) null))
  (`/Engine/EditorBlueprintResources/StandardMacros.IsValid` _returnvalue
    (:`Is Valid`
      (`/Game/InGame/Blueprints/Item/WorldItem/BP_WorldItem.StartDropPhysics` _returnvalue (`local.ImpluseDirection`))
      (return true))
    (:`Is Not Valid`
      (return false))))

(fn `UserConstructionScript`)