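; Actor component for a grid inventory that checks whether items can be placed at a hovered slot and finds items by coordinate.
; On BeginPlay it builds a coordinate slot map from the grid size and, if AutoCreate is valid, requests item IDs from the game instance.
; Placement filters by item type, then computes target cells within grid bounds, with a rotated width/height fallback.
; Item lookup scans each item's occupied coordinates.
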(event EventBeginPlay
  (CallFunction|InitGrid)
  (Variables|Widget|GetAuto%20Create
    (:then
      (CallFunction|AssignItemID (Variables|Default|GetItems)))
    (:else)))

(event EventEndPlay
  (params (EndPlayReason :type EEndPlayReason%20Enum :default "Destroyed"))
  (Default|CallComponentDestroyed)
  (Variables|Widget|SetGridWidget 0)
  (Variables|Widget|SetParentPanel 0))

(fn InitGrid
  (Utilities|Map|Clear (Variables|GridVar|GetCroodinate/Slot%20Map))
  (Variables|GridVar|SetMax%20X%20Crood (- (Variables|GridVar|GetX%20Slot%20Wide%20Size) 1))
  (Variables|GridVar|SetMax%20Y%20Crood (- (Variables|GridVar|GetY%20Slot%20High%20Size) 1))
  (for _index (range 0 (- (Variables|GridVar|GetY%20Slot%20High%20Size) 1))
    (LocalVariables|SetCurrent%20X _index)
    (for _index_2 (range 0 (- (Variables|GridVar|GetX%20Slot%20Wide%20Size) 1))
      (LocalVariables|SetCurrent%20Y _index_2)
      (Utilities|Map|Add (Variables|GridVar|GetCroodinate/Slot%20Map) (Utilities|Struct|MakeST_IndexCrood (LocalVariables|GetCurrent%20X) (LocalVariables|GetCurrent%20Y)) 0)))
  (return))

(fn AssignItemID
  (params (Items :type Array%20of%20ST%20Inventory%20Item%20Structures))
  (for (_ _array_index) Items
    (bind _id (Class|BPIGI|AssignItemID(Message) (Game|GetGameInstance)))
    (Utilities|Struct|SetmembersinST_InventoryItem (Utilities|Array|Get(acopy) Items _array_index) _id))
  (return))

(fn CalculateTargetCroodinate
  (params (StartingCrood :type ST%20Index%20Crood%20Structure) (WidthOfItem :type Integer) (HightOfItem :type Integer) (CanRotate :type Boolean) (TryVertical :type Boolean))
  (if TryVertical
    (if (and (|(((X+W)-1)<=MX) (.x StartingCrood) WidthOfItem (Variables|GridVar|GetMax%20X%20Crood)) (|(((Y+H)-1)<=MY) (.y StartingCrood) HightOfItem (Variables|GridVar|GetMax%20Y%20Crood)))
      ;[0.15 0.15 0.15 0.5] 수평 방향 아이템 추가
      (for _index (range 0 (|((X+W)-1) (.x StartingCrood) WidthOfItem))
        (LocalVariables|SetCurrentX _index)
        (for _index_2 (range 0 (|((Y+H)-1) (.y StartingCrood) HightOfItem))
          (LocalVariables|SetCurrentY _index_2)
          (if (.ReturnValue (Utilities|Map|Find (Variables|GridVar|GetCroodinate/Slot%20Map) (Utilities|Struct|MakeST_IndexCrood (LocalVariables|GetCurrentX) (LocalVariables|GetCurrentY))))
            (Utilities|Array|Add (LocalVariables|GetTargetCroodinate) (Utilities|Struct|MakeST_IndexCrood (LocalVariables|GetCurrentX) (LocalVariables|GetCurrentY)))
            (else
              ;[0.15 0.15 0.15 0.5] 수직 방향 아이템 추가
              ;;[0.15 0.15 0.15 0.5] Col
              (for _index_3 (range 0 (|((Y+W)-1) WidthOfItem (.y StartingCrood)))
                (LocalVariables|SetCurrentY _index_3)
                ;;[0.15 0.15 0.15 0.5] Row
                (for _index_4 (range 0 (|((X+H)-1) HightOfItem (.x StartingCrood)))
                  (LocalVariables|SetCurrentX _index_4)
                  (if (.ReturnValue (Utilities|Map|Find (Variables|GridVar|GetCroodinate/Slot%20Map) (Utilities|Struct|MakeST_IndexCrood (LocalVariables|GetCurrentX) (LocalVariables|GetCurrentY))))
                    (Utilities|Array|Add (LocalVariables|GetTargetCroodinate) (Utilities|Struct|MakeST_IndexCrood (LocalVariables|GetCurrentX) (LocalVariables|GetCurrentY)))
                    (else
                      (return false true 0)))))
              (return true true (LocalVariables|GetTargetCroodinate))))))
      (return true false (LocalVariables|GetTargetCroodinate)))
    (elif (not (and (|(((Y+W)-1)<=MY) WidthOfItem (.y StartingCrood) (Variables|GridVar|GetMax%20Y%20Crood)) (|(((X+H)-1)<=MX) HightOfItem (.x StartingCrood) (Variables|GridVar|GetMax%20X%20Crood))))
      (return false false 0))))

(fn FindItembyCrood
  (params (Croodinate :type ST%20Index%20Crood%20Structure))
  (for (_array_element _array_index) (Variables|Default|GetItems)
    (for _array_element_2 (.occupiedcroods _array_element)
      (if (and (== (.x _array_element_2) (.x Croodinate)) (== (.y _array_element_2) (.y Croodinate)))
        (return (Utilities|Array|Get(acopy) (Variables|Default|GetItems) _array_index))))))

(fn IteminBounds
  (params (Item :type ST%20Inventory%20Item%20Structure))
  (return (.Value (Utilities|Map|Find (Variables|Default|GetItemTypeAllowwed) (Variables|/Game/Inventory/Data/Items/PDA_ItemData.PDA_ItemData_C|GetItemType (.ItemData (Utilities|Struct|BreakST_InventoryItem Item)))))))

(fn DoesGridAcceptItem
  (params (Item :type ST%20Inventory%20Item%20Structure) (HoverdCrood :type ST%20Index%20Crood%20Structure) (TryVertical :type Boolean))
  (bind (___of_slot_wide ___of_slot_high) (CallFunction|GetItemSize (.itemdata Item)))
  (if (CallFunction|IteminBounds Item)
    (bind (_withinbound _rotate _croodinate) (CallFunction|CalculateTargetCroodinate HoverdCrood ___of_slot_wide ___of_slot_high (Variables|/Game/Inventory/Data/Items/PDA_ItemData.PDA_ItemData_C|GetCan%20Rotate (.itemdata Item)) TryVertical))
    (return _withinbound _rotate _croodinate)
    (else
      (CallFunction|DebugErrorPrintString "아이템 못 들어감" self)
      (return false false 0))))

(fn GetItemSize
  (params (ItemData :type PDA%20Item%20Data%20Object%20Reference))
  (return (Variables|/Game/Inventory/Data/Items/PDA_ItemData.PDA_ItemData_C|Get#%20of%20Slot%20Wide ItemData) (Variables|/Game/Inventory/Data/Items/PDA_ItemData.PDA_ItemData_C|Get#%20of%20Slot%20High ItemData)))